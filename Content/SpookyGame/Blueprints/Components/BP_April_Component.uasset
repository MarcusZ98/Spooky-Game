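; BP_April_Component is the hint component for April, playing audio hints based on the player's progress in Levels 2 and 3.
; GiveHint requires that the player can interact and no dialogue is active, then selects a sound from the current level name and GameState's level state.
; PlayHintSound plays it in 2D, or only stops the current hint if one is already playing.
; The Level 2 hint has no sound assigned.
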(event Custom|Give%20Hint
  (params (DM :type BP%20Dialogue%20Manager%20Object%20Reference) (PlayerREF :type BP%20SG%20Player%20Object%20Reference))
  (bind _output_get (Variables|Default|SetDM DM))
  (if (Variables|/Game/SpookyGame/Blueprints/Player/BP_SG_Player.BP_SG_Player_C|GetCanInteract PlayerREF)
    (if (not (Variables|/Game/SpookyGame/Blueprints/Dialogue/BP_DialogueManager.BP_DialogueManager_C|GetIsDialogueActive _output_get))
      (bind _returnvalue (Game|GetCurrentLevelName true))
      (switch string _returnvalue
        (:Level_2
          (switch Utilities|FlowControl|Switch|SwitchonLevel_2_States (Variables|/Game/SpookyGame/Blueprints/FrameWork/BP_SG_GameState.BP_SG_GameState_C|GetLevel2States (Variables|Default|GetGameState))
            (:NewEnumerator0
              (CallFunction|PlayHintSound))))
        (:Level_3
          (switch Utilities|FlowControl|Switch|SwitchonLevel_3_States (Variables|/Game/SpookyGame/Blueprints/FrameWork/BP_SG_GameState.BP_SG_GameState_C|GetLevel3States (Variables|Default|GetGameState))
            (:NewEnumerator0
              (CallFunction|PlayHintSound "/Game/SpookyGame/Audio/Baby-room_lvl3_Audio/SFX_Voice-Lines/SFX_April_Hints/SFX_lvl3_Hint_SoundWaves/SFX_lvl3_H1_MaybeWeCanCalmHim.SFX_lvl3_H1_MaybeWeCanCalmHim"))
            (:NewEnumerator1
              (CallFunction|PlayHintSound "/Game/SpookyGame/Audio/Baby-room_lvl3_Audio/SFX_Voice-Lines/SFX_Scripted-Dialogue/SFX_Scripted-Dialogue_Sound-Wave/SFX_lvl3_DidYouNoticeTheCabinet.SFX_lvl3_DidYouNoticeTheCabinet"))
            (:NewEnumerator2
              (CallFunction|PlayHintSound "/Game/SpookyGame/Audio/Baby-room_lvl3_Audio/SFX_Voice-Lines/SFX_April_Hints/SFX_lvl3_H6_TheCabinetIsOpen_Cue.SFX_lvl3_H6_TheCabinetIsOpen_Cue"))))))
    (else
      (Development|PrintString "April can't give hint right now" true true "(R=0.615000,G=0.000000,B=0.355016,A=1.000000)" 2.0 "1"))))

(event EventBeginPlay
  (bind _asbp_sg_game_state (Utilities|Casting|CastToBP_SG_GameState (Game|GetGameState)))
  (Variables|Default|SetGameState _asbp_sg_game_state))

(event EventTick
  (params (DeltaSeconds :type Float%20%28single-precision%29)))

(fn PlayHintSound
  (params (DialogueSound :type Sound%20Base%20Object%20Reference))
  (Utilities|IsValid (Variables|Default|GetHintSound)
    (:Is%20Valid
      (if (Audio|Components|Audio|IsPlaying (Variables|Default|GetHintSound))
        (Audio|Components|Audio|Stop (Variables|Default|GetHintSound))
        (else
          (bind _returnvalue (Audio|SpawnSound2D DialogueSound 1.0 1.0 0.0 0 :!label _label))
          (Variables|Default|SetHintSound _returnvalue)
          (return))))
    (:Is%20Not%20Valid
      (goto _label))))