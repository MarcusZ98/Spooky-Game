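; Player component that plays a descriptive sound for the object the player's camera is looking at.
; SoundDescriptionEvent line-traces 500 units along the camera's forward vector, with debug drawing, for configured object types.
; PlayDescriptionSound looks up the hit actor's class in SoundMapping, prints its name, plays the 2D sound and returns its duration.
; A DoOnce, reset after a Delay of that duration, keeps descriptions from overlapping.
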(event Custom|Sound%20Description%20Event
  (params (Camera :type Camera%20Component%20Object%20Reference))
  (bind _returnvalue (Transformation|GetWorldLocation Camera))
  ;[1 0.2956 0.7464] Play descriptive sound event
  (Utilities|FlowControl|DoOnce false :!label _label
    (:Completed
      (bind _outhit (Collision|LineTraceForObjects _returnvalue (+ _returnvalue (* (Math|Vector|GetForwardVector Camera) 5e+02)) (Variables|Default|GetObjectsToFind) false 0 "ForDuration"))
      (bind _soundduration (CallFunction|PlayDescriptionSound (.hitactor _outhit)))
      (Utilities|FlowControl|Delay _soundduration)
      (goto _label Reset))))

(event EventBeginPlay)

(event EventTick
  (params (DeltaSeconds :type Float%20%28single-precision%29)))

(fn PlayDescriptionSound
  (params (Actor%20Hit :type Actor%20Object%20Reference))
  (bind _returnvalue (Utilities|GetClass Actor%20Hit))
  (bind _soundmapping (Variables|Default|GetSoundMapping))
  (bind (_value _returnvalue_2) (Utilities|Map|Find _soundmapping _returnvalue))
  (if _returnvalue_2
    (Development|PrintString (Utilities|String|Append "Description Sound: " (Utilities|GetDisplayName Actor%20Hit)) true true "(R=0.315984,G=0.000000,B=1.000000,A=1.000000)")
    (Audio|PlaySound2D _value 1.0 1.0 0.0 0 0)
    (return (Variables|/Script/Engine.SoundBase|GetDuration _value))))