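; BP_MainMenuComponent is a component that creates and controls the main menu widget.
; It creates the MainMenu widget on BeginPlay and keeps a reference.
; OpenMenu adds that widget to the viewport and switches to game-and-UI input with the mouse locked.
; CloseMenu stops its sounds, resets the Start and Settings panels, removes all widgets and restores game-only input.
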(event EventBeginPlay
  (bind _returnvalue (UserInterface|CreateWidget "/Game/SpookyGame/Blueprints/Widgets/MainMenu.MainMenu_C" (Game|GetPlayerController 0)))
  (Variables|Default|SetWidgetRef _returnvalue))

(event EventTick
  (params (DeltaSeconds :type Float%20%28single-precision%29)))

(fn OpenMenu
  (bind _widgetref (Variables|Default|GetWidgetRef))
  (Utilities|IsValid _widgetref
    (:Is%20Valid
      (Development|PrintString "Already exist")
      (UserInterface|Viewport|AddtoViewport _widgetref 0)
      (Input|SetInputModeGameandUI (Game|GetPlayerController 0) _widgetref "LockAlways" true true))))

(fn CloseMenu
  (bind _widgetref (Variables|Default|GetWidgetRef))
  (Utilities|IsValid _widgetref
    (:Is%20Valid
      (Default|StopAllSounds _widgetref)
      (Variables|/Script/UMG.Widget|SetVisibility (Variables|/Game/SpookyGame/Blueprints/Widgets/MainMenu.MainMenu_C|GetSettings _widgetref) "Hidden")
      (Variables|/Script/UMG.Widget|SetVisibility (Variables|/Game/SpookyGame/Blueprints/Widgets/MainMenu.MainMenu_C|GetStart _widgetref) "Visible")
      (Viewport|RemoveAllWidgets)
      (Input|SetInputModeGameOnly (Game|GetPlayerController 0) true))))