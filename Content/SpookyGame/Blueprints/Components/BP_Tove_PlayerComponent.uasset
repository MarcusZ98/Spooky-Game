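; Player component for Tove that handles the hint button and gates interaction with objects.
; Hints play a sound from the target inside a timed audio focus event.
; The piano puzzle pawn and music box are registered as invalid interactables, blocked from the proximity sound and interaction once the puzzle is completed.
; Allowed presses, subject to the player's CanInteract flag, forward TriggerEventMessage to the current object.
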(event Custom|Hint%20Button
  (params (Target :type BP%20April%20Object%20Reference))
  ;[1 0.3744 0.6006] Hint button
  (if (Variables|/Game/SpookyGame/Blueprints/NPC/BP_April.BP_April_C|GetCanGiveHint Target)
    (bind (_sound_duration _hint_sound) (Default|PlaySound Target))
    (CallFunction|BeginFocusEvent _hint_sound true 0.2 0.0)
    (Utilities|FlowControl|Delay _sound_duration)
    (CallFunction|ExitFocusEvent 0.2)
    (Development|PrintString "Exit focus on hint" true true "(R=0.414927,G=1.000000,B=0.000000,A=1.000000)")
    (else
      (Development|PrintString "April can't give hint!" true true "(R=1.000000,G=0.000000,B=0.075015,A=1.000000)"))))

(event Custom|Invalid%20interactable%20set%20add
  ;[1 0.6739 0.3204] Add invalid interactables
  (bind _returnvalue (Actor|GetActorOfClass "/Game/SpookyGame/Blueprints/Objects/BP_PuzzlePawn_Piano.BP_PuzzlePawn_Piano_C"))
  (bind _returnvalue_2 (Actor|GetActorOfClass "/Game/SpookyGame/Blueprints/Objects/BP_InteractableObject_MusicBox.BP_InteractableObject_MusicBox_C"))
  (Utilities|Set|AddItems (Variables|Default|GetInvalidInteractables) (Utilities|Array|MakeArray _returnvalue_2 _returnvalue)))

(event Custom|Is%20Close%20To%20Interactable%20Object
  (params (CurrentInteractableObject :type Actor%20Object%20Reference) (PuzzleCompleted :type Boolean))
  ;[1 0.4843 0.8598] Check if we should play interact sound
  (if PuzzleCompleted
    (if (Utilities|Set|Contains (Variables|Default|GetInvalidInteractables) CurrentInteractableObject)
      (Development|PrintString (Utilities|String|Append "Can't interact with:" (Utilities|GetDisplayName CurrentInteractableObject)) true true "(R=1.000000,G=0.023625,B=0.000000,A=1.000000)")
      (else
        (Audio|PlaySound2D "/Game/SpookyGame/Audio/All_Rooms/SFX/SFX_Interact_Active.SFX_Interact_Active" 1.0 1.0 0.0 0 0 :!label _label)
        (Development|PrintString (Utilities|String|Append "Can interact with: " (Utilities|GetDisplayName CurrentInteractableObject)) true true "(R=0.426765,G=1.000000,B=0.000000,A=1.000000)")))
    (else
      (goto _label))))

(event Custom|Press%20interact
  (params (PuzzleComplete :type Boolean) (CurrentInteractable :type Actor%20Object%20Reference) (PlayerREF :type BP%20SG%20Player%20Object%20Reference))
  (if (Variables|/Game/SpookyGame/Blueprints/Player/BP_SG_Player.BP_SG_Player_C|GetCanInteract PlayerREF)
    (if PuzzleComplete
      (if (Utilities|Set|Contains (Variables|Default|GetInvalidInteractables) CurrentInteractable)
        (Development|PrintString "Can't interact with this object" true true "(R=1.000000,G=0.000000,B=0.018112,A=1.000000)")
        (else
          (Class|BPIInteractable|TriggerEvent(Message) CurrentInteractable PlayerREF :!label _label)
          (Development|PrintString (Utilities|String|Append "Interacting with:" (Utilities|GetDisplayName CurrentInteractable)))))
      (else
        (goto _label)))
    (else
      (Development|PrintString "Can't interact right now" true true "(R=1.000000,G=0.162241,B=0.751155,A=1.000000)"))))

(event EventBeginPlay)

(event EventTick
  (params (DeltaSeconds :type Float%20%28single-precision%29)))

(fn IsInvalidInteractable
  (params (CurrentInteractable :type Actor%20Object%20Reference) (PuzzleCompleted :type Boolean) (InvalidInteractables :type Set%20of%20Actor%20Object%20References))
  (return (Utilities|Set|Contains InvalidInteractables CurrentInteractable)))