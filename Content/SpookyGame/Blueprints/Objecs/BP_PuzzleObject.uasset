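; BP_PuzzleObject is a puzzle actor, apparently a base for puzzles, that handles swapping player controls between normal play and puzzle interaction.
; ChangePlayerController uses a FlipFlop to swap the default and puzzle Enhanced Input mapping contexts on player 0, alternating on each call.
; PuzzleCompleted is an empty stub, and the event graph holds no active logic.
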(event EventBeginPlay
  (|CallParentFunction) ; This node is disabled and will not be called.\nDrag off pins to build functionality.
)

(event Collision|EventActorBeginOverlap
  (params (OtherActor :type Actor%20Object%20Reference))
  (|CallParentFunction OtherActor) ; This node is disabled and will not be called.\nDrag off pins to build functionality.
)

(event EventTick
  (params (DeltaSeconds :type Float%20%28single-precision%29))
  (|CallParentFunction DeltaSeconds) ; This node is disabled and will not be called.\nDrag off pins to build functionality.
)

(fn ConstructionScript
  (|CallParentFunction))

(fn PuzzleCompleted)

(fn ChangePlayerController
  (bind _returnvalue (Game|GetPlayerController 0))
  (bind _returnvalue_2 (PlayerController|LocalPlayerSubsystems|GetEnhancedInputLocalPlayerSubsystem _returnvalue))
  ;[1 1 1] Switches between controlls
  (Utilities|FlowControl|FlipFlop
    (:A
      ;;[1 1 1] Sets Puzzle Controll
      (Input|RemoveMappingContext _returnvalue_2 (Variables|Default|GetPlayerDefaultMapping) "(bIgnoreAllPressedKeysUntilRelease=True,bForceImmediately=False,bNotifyUserSettings=False)")
      (Input|AddMappingContext _returnvalue_2 (Variables|Default|GetPuzzleInputMapping) 0 "(bIgnoreAllPressedKeysUntilRelease=True,bForceImmediately=False,bNotifyUserSettings=False)"))
    (:B
      ;;[1 1 1] Sets Player Deafult Controll
      (Input|RemoveMappingContext _returnvalue_2 (Variables|Default|GetPuzzleInputMapping) "(bIgnoreAllPressedKeysUntilRelease=True,bForceImmediately=False,bNotifyUserSettings=False)")
      (Input|AddMappingContext _returnvalue_2 (Variables|Default|GetPlayerDefaultMapping) 0 "(bIgnoreAllPressedKeysUntilRelease=True,bForceImmediately=False,bNotifyUserSettings=False)"))))