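; April is an NPC that runs a state machine and gives the player narrative hints.
; Init caches the player and enters the preset CurrentState, disabling tick if either is missing.
; Each tick, the state either ticks or hands over to the next state it supplies, unless PlayerIsPossessed teleports April to the piano instead.
; PlaySound gives the current state's hint sound when audio is idle.
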(event EventBeginPlay
  (|CallParentFunction)
  ;[1 1 1] Initialize and disable tick if it fails
  (bind _success (CallFunction|Init))
  (Actor|Tick|SetActorTickEnabled _success))

(event EventTick
  (params (DeltaSeconds :type Float%20%28single-precision%29))
  (|CallParentFunction DeltaSeconds)
  (if (Variables|Default|GetPlayerIsPossessed) ; Check if player is in alt controls
    (Transformation|Teleport "510.000000,30.000000,0.000000" "0, 0, 0") ; Teleport to piano
    (elif (Default|ShouldTransitionState (Variables|Default|GetCurrentState))
      (bind _next_state (Default|GetNextState (Variables|Default|GetCurrentState)))
      (Default|TransitiontoState _next_state self (Variables|Default|GetPlayer))
      (Variables|Default|SetCurrentState _next_state)
      (else
        (Default|TickState (Variables|Default|GetCurrentState) DeltaSeconds)))))

(fn ConstructionScript
  (|CallParentFunction))

(fn Init
  (bind _output_get (Variables|Default|SetPlayer (Game|GetPlayerCharacter 0)))
  (if (Utilities|IsValid _output_get)
    (if (Utilities|IsValid (Variables|Default|GetCurrentState))
      (Default|TransitiontoState (Variables|Default|GetCurrentState) self (Variables|Default|GetPlayer))
      (return true)
      (else
        (Development|PrintString "No initial state for april. Please set initial state in \"CurrentState\"." true true "(R=0.000000,G=0.660000,B=1.000000,A=1.000000)" 25.0)))
    (else
      (Development|PrintString "April couldnt find player character.")))
  (return false))

(fn PlaySound
  (bind _currentstate (Variables|Default|GetCurrentState))
  (bind _hintsound (Default|GetHintSound _currentstate))
  (if (not (Audio|Components|Audio|IsPlaying (Variables|Default|GetAudio)))
    (Development|PrintString "Focus on hint" true true "(R=1.000000,G=0.000000,B=0.750000,A=1.000000)")
    (Default|GiveNarrativeHint self _hintsound)
    (return (Variables|/Script/Engine.SoundBase|GetDuration _hintsound) _hintsound)))