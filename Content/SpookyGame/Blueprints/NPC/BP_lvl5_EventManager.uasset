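; Level 5 event manager that triggers that level's story dialogue through the level's BP_DialogueManager.
; On BeginPlay it finds and caches the dialogue manager, then plays the intro dialogue after a short delay.
; CrystalOrbEnding and KillApril events play the ending and April-kill dialogue assets.
; All three route through a SetPlayDialogue helper that sets the dialogue asset and starts it.
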(event Custom|CrystalOrbEnding
  (CallFunction|SetPlayDialogue (Variables|Default|GetDialogue_Manager) "/Game/SpookyGame/Blueprints/Dialogue/Level_5_Dialogue/DA_lvl5_Ending_Dialogue.DA_lvl5_Ending_Dialogue"))

(event Custom|KillApril
  (CallFunction|SetPlayDialogue (Variables|Default|GetDialogue_Manager) "/Game/SpookyGame/Blueprints/Dialogue/Level_5_Dialogue/DA_lvl5_KillApril_Dialogue.DA_lvl5_KillApril_Dialogue"))

(event EventBeginPlay
  (bind _returnvalue (Actor|GetActorOfClass "/Game/SpookyGame/Blueprints/Dialogue/BP_DialogueManager.BP_DialogueManager_C"))
  (Utilities|IsValid _returnvalue
    (:Is%20Valid
      (bind _output_get (Variables|Default|SetDialogue_Manager _returnvalue))
      (Utilities|FlowControl|Delay 0.3)
      (CallFunction|SetPlayDialogue _output_get "/Game/SpookyGame/Blueprints/Dialogue/Level_5_Dialogue/DA_lvl5_Init_Dialogue.DA_lvl5_Init_Dialogue"))))

(fn ConstructionScript)

(fn SetPlayDialogue
  (params (DM :type BP%20Dialogue%20Manager%20Object%20Reference) (DialogueSound :type BP%20Dialogue%20Object%20Reference))
  (Default|SetDialogue DM DialogueSound)
  (Default|StartDialogue DM)
  (return))