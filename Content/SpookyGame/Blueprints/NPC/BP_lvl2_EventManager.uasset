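; BP_lvl2_EventManager drives level 2's scripted story beats by triggering dialogue and advancing the level state.
; On BeginPlay it caches the BP_DialogueManager, plays the intro dialogue after a short delay and sets the initial Level2States on BP_SG_GameState.
; Radio, door, shipwheel and break-glass events play dialogue via SetPlayDialogue; radio and shipwheel also advance the state.
; The first three skip when passed an already-interacted flag.
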(event Custom|InteractedWithRadio
  (params (HasInteractedWithRadio :type Boolean))
  (if HasInteractedWithRadio
    (Development|PrintString "skipped")
    (else
      (CallFunction|SetPlayDialogue (Variables|Default|GetDialogue_Manager) "/Game/SpookyGame/Blueprints/Dialogue/Level_2_Dialogue/DA_lvl2_RadioInteract_Dialogue.DA_lvl2_RadioInteract_Dialogue")
      (bind _asbp_sg_game_state (Utilities|Casting|CastToBP_SG_GameState (Game|GetGameState)))
      (Variables|/Game/SpookyGame/Blueprints/FrameWork/BP_SG_GameState.BP_SG_GameState_C|SetLevel2States _asbp_sg_game_state "NewEnumerator1"))))

(event Custom|StartScriptedDoorEvent
  (params (HasInteractedWithDoor :type Boolean))
  (if HasInteractedWithDoor
    (Development|PrintString "skipped" true true "(R=0.000000,G=0.660000,B=1.000000,A=1.000000)" 2.0 "1")
    (else
      (CallFunction|SetPlayDialogue (Variables|Default|GetDialogue_Manager) "/Game/SpookyGame/Blueprints/Dialogue/Level_2_Dialogue/DA_lvl2_DoorInteact_Dialogue.DA_lvl2_DoorInteact_Dialogue"))))

(event Custom|ScriptedShipwheelEvent
  (params (HasInteractedWithWheel :type Boolean))
  (if HasInteractedWithWheel
    (Development|PrintString "Skipped" true true "(R=0.000000,G=0.660000,B=1.000000,A=1.000000)" 2.0 "1")
    (else
      (CallFunction|SetPlayDialogue (Variables|Default|GetDialogue_Manager) "/Game/SpookyGame/Blueprints/Dialogue/Level_2_Dialogue/DA_lvl2_Shipwheel-Inteact_Dialogue.DA_lvl2_Shipwheel-Inteact_Dialogue")
      (bind _asbp_sg_game_state (Utilities|Casting|CastToBP_SG_GameState (Game|GetGameState)))
      (Variables|/Game/SpookyGame/Blueprints/FrameWork/BP_SG_GameState.BP_SG_GameState_C|SetLevel2States _asbp_sg_game_state "NewEnumerator2"))))

(event Custom|BreakGlassScriptedEvent
  (CallFunction|SetPlayDialogue (Variables|Default|GetDialogue_Manager) "/Game/SpookyGame/Blueprints/Dialogue/Level_2_Dialogue/DA_lvl2_BreakGlass_Dialogue.DA_lvl2_BreakGlass_Dialogue"))

(event EventBeginPlay
  (bind _returnvalue (Actor|GetActorOfClass "/Game/SpookyGame/Blueprints/Dialogue/BP_DialogueManager.BP_DialogueManager_C"))
  (Utilities|IsValid _returnvalue
    (:Is%20Valid
      (bind _output_get (Variables|Default|SetDialogue_Manager _returnvalue))
      (Utilities|FlowControl|Delay 0.3)
      (CallFunction|SetPlayDialogue _output_get "/Game/SpookyGame/Blueprints/Dialogue/Level_2_Dialogue/DA_lvl2_Init_Dialogue.DA_lvl2_Init_Dialogue")
      (bind _asbp_sg_game_state (Utilities|Casting|CastToBP_SG_GameState (Game|GetGameState)))
      (Variables|/Game/SpookyGame/Blueprints/FrameWork/BP_SG_GameState.BP_SG_GameState_C|SetLevel2States _asbp_sg_game_state "NewEnumerator0"))))

(fn ConstructionScript)

(fn SetPlayDialogue
  (params (DM :type BP%20Dialogue%20Manager%20Object%20Reference) (DialogueSound :type BP%20Dialogue%20Object%20Reference))
  (Default|SetDialogue DM DialogueSound)
  (Default|StartDialogue DM)
  (return))