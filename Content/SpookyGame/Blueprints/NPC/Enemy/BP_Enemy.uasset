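; BP_Enemy is an enemy NPC that switches the player into combat on contact.
; When the player character overlaps its capsule, a DoOnce spawns a BP_Combat actor at the player's transform and has the player controller possess it.
; One second after BeginPlay it prints its AI controller's name and a marker string as debug output.
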(event OnComponentBeginOverlap(CapsuleCollider)
  (params (OverlappedComponent :type Primitive%20Component%20Object%20Reference) (OtherActor :type Actor%20Object%20Reference) (OtherComp :type Primitive%20Component%20Object%20Reference) (OtherBodyIndex :type Integer) (bFromSweep :type Boolean) (SweepResult :type Hit%20Result%20Structure%20%28by%20ref%29))
  (if (== OtherActor (Game|GetPlayerCharacter 0))
    (Utilities|FlowControl|DoOnce false
      (:Completed
        (bind _returnvalue (Game|SpawnActorfromClass "/Game/SpookyGame/Blueprints/Objects/BP_Combat.BP_Combat_C" (Transformation|GetActorTransform (Game|GetPlayerCharacter 0)) "Undefined" "MultiplyWithRoot" 0 0))
        (Pawn|Possess (Game|GetPlayerController 0) _returnvalue)))))

(event EventBeginPlay
  (Utilities|FlowControl|Delay 1.0)
  (Development|PrintString (Utilities|GetDisplayName (AI|GetAIController 0)))
  (Development|PrintString "&&&&&&&"))

(fn ConstructionScript
  (|CallParentFunction))