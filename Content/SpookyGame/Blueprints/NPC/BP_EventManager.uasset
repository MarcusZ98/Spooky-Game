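; BP_EventManager is an event manager that, as wired, only finds and caches the BP_April actor on BeginPlay.
; It also holds a disconnected, never-executed dialogue sequence timed by delays and sound durations.
; That sequence wraps a line in a scripted dialogue event, then plays the level 3 "LetsTakeALookAround" cue at April's location while temporarily disabling her hints.
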(event EventBeginPlay
  (bind _returnvalue (Actor|GetActorOfClass "/Game/SpookyGame/Blueprints/NPC/BP_April.BP_April_C"))
  (Variables|Default|SetApril _returnvalue))

(event Collision|EventActorBeginOverlap
  (params (OtherActor :type Actor%20Object%20Reference)))

(event EventTick
  (params (DeltaSeconds :type Float%20%28single-precision%29)))

(fn ConstructionScript)