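; April's idle NPC state for Level 3, in which the April pawn keeps turning to face the player on the horizontal plane.
; It transitions once the player moves farther than a minimum 2D distance from the interactable location.
; It then scores each possible next state by the dot product of player facing and direction to that state's target, picking the best valid match.
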(fn ShouldTransitionState
  (bind _playerpawn (Variables|Default|GetPlayerPawn))
  (bind _interactable_location (Variables|Default|GetInteractable%20Location))
  (bind _playerpawn_2 (Variables|Default|GetPlayerPawn))
  (bind _returnvalue (Transformation|GetActorLocation _playerpawn))
  (if (> (Math|Vector|Distance(Vector) (Math|Vector|MakeVector (.x _returnvalue) (.y _returnvalue) 0.0) (Math|Vector|MakeVector (.x _interactable_location) (.y _interactable_location) 0.0)) (Variables|Default|GetMinDistanceToInteractableActor)) ; Only check next state when we should transition
    (LocalVariables|SetBest%20Dot -1.0) ; Reset dot
    (for _array_element (Variables|Default|GetPossibleNextStates)
      ;[1 1 1] If better than previous best -> Set as new best
      (if (> (Math|Vector|DotProduct (Math|Vector|GetForwardVector (Math|Rotator|FindLookatRotation (Transformation|GetActorLocation _playerpawn_2) (Variables|/Game/SpookyGame/Blueprints/NPC/DataAssets/Level_3/BP_AprilMoveState.BP_AprilMoveState_C|GetTargetLocation _array_element))) (Transformation|GetActorForwardVector _playerpawn_2)) (LocalVariables|GetBest%20Dot))
        (LocalVariables|SetBest%20Dot (Math|Vector|DotProduct (Math|Vector|GetForwardVector (Math|Rotator|FindLookatRotation (Transformation|GetActorLocation _playerpawn_2) (Variables|/Game/SpookyGame/Blueprints/NPC/DataAssets/Level_3/BP_AprilMoveState.BP_AprilMoveState_C|GetTargetLocation _array_element))) (Transformation|GetActorForwardVector _playerpawn_2)))
        (LocalVariables|SetBest%20State _array_element)))
    (return (Utilities|IsValid (LocalVariables|GetBest%20State)) (LocalVariables|GetBest%20State))
    (else
      (return false self))))

(fn TickState
  (params (DeltaSeconds :type Float%20%28double-precision%29))
  (bind _playerpawn (Variables|Default|GetPlayerPawn))
  (bind _aprilpawn (Variables|Default|GetAprilPawn))
  (bind _returnvalue (Transformation|GetActorLocation _aprilpawn))
  (bind _returnvalue_2 (Transformation|GetActorLocation _playerpawn))
  (Transformation|SetActorRotation _aprilpawn (Math|Rotator|FindLookatRotation (Math|Vector|MakeVector (.x _returnvalue) (.y _returnvalue) 0.0) (Math|Vector|MakeVector (.x _returnvalue_2) (.y _returnvalue_2) 0.0))) ; Look at player
)