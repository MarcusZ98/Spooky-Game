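; April move state that moves the April NPC pawn toward a target location in Level 3.
; Each tick it interpolates the pawn's location toward the target using the pawn's MoveSpeed and snaps its rotation to face the target.
; It signals a transition to the configured next state once horizontal distance to the target, ignoring height, drops below StopDistance.
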(fn ShouldTransitionState
  (bind _targetlocation (Variables|Default|GetTargetLocation))
  (bind _aprilpawn (Variables|Default|GetAprilPawn))
  (bind _returnvalue (Transformation|GetActorLocation _aprilpawn))
  (return (< (Math|Vector|Distance(Vector) (Math|Vector|MakeVector (.x _returnvalue) (.y _returnvalue) 0.0) (Math|Vector|MakeVector (.x _targetlocation) (.y _targetlocation) 0.0)) (Variables|Default|GetStop%20distance)) (Variables|Default|GetNext%20State)))

(fn TickState
  (params (DeltaSeconds :type Float%20%28double-precision%29))
  (bind _aprilpawn (Variables|Default|GetAprilPawn))
  (Transformation|SetActorLocationAndRotation _aprilpawn (Math|Interpolation|VInterpTo (Transformation|GetActorLocation _aprilpawn) (Variables|Default|GetTargetLocation) DeltaSeconds (Variables|/Game/SpookyGame/Blueprints/NPC/BP_April.BP_April_C|GetMoveSpeed _aprilpawn)) (Math|Rotator|FindLookatRotation (Transformation|GetActorLocation _aprilpawn) (Variables|Default|GetTargetLocation))))