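; Level 3 event manager that triggers dialogue as the player progresses through the baby, puzzle and teddy story beats.
; On BeginPlay it finds the level's BP_DialogueManager and, after a short delay, plays the intro dialogue.
; Progress events each pass their dialogue asset to SetPlayDialogue, which sets and starts it on the manager.
; The baby interaction line is skipped, with a debug print, if the passed flag says it already happened.
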(event Custom|PlayerHasInteractedWithBaby
  (params (HasInteractedWithBaby :type Boolean))
  (if HasInteractedWithBaby
    (Development|PrintString "skipped")
    (else
      (CallFunction|SetPlayDialogue (Variables|Default|GetDialogue_Manager) "/Game/SpookyGame/Blueprints/Dialogue/Level_3_Dialogue/DA_lvl3_Interacted-With-Baby_Dialogue.DA_lvl3_Interacted-With-Baby_Dialogue"))))

(event Custom|PlayerHasCompletedPuzzle
  (CallFunction|SetPlayDialogue (Variables|Default|GetDialogue_Manager) "/Game/SpookyGame/Blueprints/Dialogue/Level_3_Dialogue/DA_lvl3_Completed-Puzzle_Dialogue1.DA_lvl3_Completed-Puzzle_Dialogue1"))

(event Custom|PlayerHasTeddy
  (CallFunction|SetPlayDialogue (Variables|Default|GetDialogue_Manager) "/Game/SpookyGame/Blueprints/Dialogue/Level_3_Dialogue/DA_lvl3_HasTeddy_Dialogue.DA_lvl3_HasTeddy_Dialogue"))

(event Custom|PlayerHasGivenTeddy
  (CallFunction|SetPlayDialogue (Variables|Default|GetDialogue_Manager) "/Game/SpookyGame/Blueprints/Dialogue/Level_3_Dialogue/DA_lvl3_HasGivenTeddy_Dialogue.DA_lvl3_HasGivenTeddy_Dialogue"))

(event EventBeginPlay
  (bind _returnvalue (Actor|GetActorOfClass "/Game/SpookyGame/Blueprints/Dialogue/BP_DialogueManager.BP_DialogueManager_C"))
  (Utilities|IsValid _returnvalue
    (:Is%20Valid
      (bind _output_get (Variables|Default|SetDialogue_Manager _returnvalue))
      (Utilities|FlowControl|Delay 0.3)
      (CallFunction|SetPlayDialogue _output_get "/Game/SpookyGame/Blueprints/Dialogue/Level_3_Dialogue/DA_lvl3_Init_Dialogue.DA_lvl3_Init_Dialogue"))))

(fn ConstructionScript)

(fn SetPlayDialogue
  (params (DM :type BP%20Dialogue%20Manager%20Object%20Reference) (DialogueSound :type BP%20Dialogue%20Object%20Reference))
  (Default|SetDialogue DM DialogueSound)
  (Default|StartDialogue DM)
  (return))