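; Dialogue manager that plays voiced conversations between April and Zac, locking player movement and starting the current dialogue at BeginPlay.
; StartDialogue moves an audio component to the speaker, plays the line, then schedules itself or ExitDialogue with duration-based timers.
; SkipVoiceLine cuts to the next line or exits.
; ExitDialogue stops audio, restores walking, resets the index, logs the dialogue to BP_NarrativeLog and repossesses the player.
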(event EventBeginPlay
  (bind _asbp_sg_player (Utilities|Casting|CastToBP_SG_Player (Game|GetPlayerCharacter 0))
    (:then
      (Variables|Default|SetPlayer _asbp_sg_player)
      (bind _returnvalue (Actor|GetActorOfClass "/Game/SpookyGame/Blueprints/NPC/BP_April.BP_April_C"))
      (Variables|Default|SetApril _returnvalue)
      (bind _returnvalue_2 (Actor|GetActorOfClass "/Game/SpookyGame/Blueprints/Dialogue/BP_NarrativeLog.BP_NarrativeLog_C"))
      (Variables|Default|SetBP_NarrativeLog _returnvalue_2)
      (Utilities|FlowControl|DelayUntilNextTick)
      (CallFunction|StartDialogue))
    (:CastFailed
      (Development|PrintString "Can't find player"))))

(event Collision|EventActorBeginOverlap
  (params (OtherActor :type Actor%20Object%20Reference)))

(event EventTick
  (params (DeltaSeconds :type Float%20%28single-precision%29)))

(fn ConstructionScript)

(fn LockPlayer
  (Pawn|Components|CharacterMovement|DisableMovement (Variables|/Script/Engine.Character|GetCharacterMovement (Variables|Default|GetPlayer))))

(fn UnlockPlayer
  (Pawn|Components|CharacterMovement|SetMovementMode (Variables|/Script/Engine.Character|GetCharacterMovement (Variables|Default|GetPlayer)) "MOVE_Walking" 0))

(fn StartDialogue
  (bind _audio (Variables|Default|GetAudio))
  (bind _audio_2 (Variables|Default|GetAudio))
  (bind _currentdialogue (Variables|Default|GetCurrentDialogue))
  (bind _dialoguecurrentindex (Variables|Default|GetDialogueCurrentIndex))
  (bind _dialogue (Variables|/Game/SpookyGame/Blueprints/Dialogue/BP_Dialogue.BP_Dialogue_C|GetDialogue _currentdialogue))
  (bind _output (Utilities|Array|Get(acopy) _dialogue _dialoguecurrentindex))
  (bind _voiceline (Variables|/Game/SpookyGame/Blueprints/Dialogue/BP_VoiceLine.BP_VoiceLine_C|GetVoiceLine _output))
  (if (>= (Variables|Default|GetDialogueCurrentIndex) (Utilities|Array|Length (Variables|/Game/SpookyGame/Blueprints/Dialogue/BP_Dialogue.BP_Dialogue_C|GetDialogue (Variables|Default|GetCurrentDialogue))))
    (Development|PrintString "Out Of bounds")
    (CallFunction|UnlockPlayer)
    (else
      (Variables|Default|SetIsDialogueActive true)
      (CallFunction|LockPlayer)
      (switch string (Variables|/Game/SpookyGame/Blueprints/Dialogue/BP_VoiceLine.BP_VoiceLine_C|GetSpeaker _output)
        (:April
          (Transformation|SetWorldLocation _audio (Transformation|GetActorLocation (Variables|Default|GetApril)) false false)
          (Audio|Components|Audio|SetSound _audio _voiceline)
          (Audio|Components|Audio|Play _audio 0.0))
        (:Zac
          (Transformation|SetWorldLocation _audio_2 (Transformation|GetActorLocation (Variables|Default|GetPlayer)) false false)
          (Audio|Components|Audio|SetSound _audio_2 _voiceline)
          (Audio|Components|Audio|Play _audio_2 0.0)))
      (Math|Integer|IncrementInt (Variables|Default|GetDialogueCurrentIndex)
        (:%20%20
          (if (< (Variables|Default|GetDialogueCurrentIndex) (Utilities|Array|Length (Variables|/Game/SpookyGame/Blueprints/Dialogue/BP_Dialogue.BP_Dialogue_C|GetDialogue (Variables|Default|GetCurrentDialogue))))
            (Development|PrintString "Voiceline")
            (bind _returnvalue (Utilities|Time|SetTimerbyFunctionName 0 "StartDialogue" (+ (Variables|/Script/Engine.SoundBase|GetDuration _voiceline) (Variables|Default|GetTimeBetweenVoiceLines))))
            (Variables|Default|SetDialogueTimerHandle _returnvalue)
            (else
              (Development|PrintString "Dialogue is finished")
              (bind _returnvalue_2 (Utilities|Time|SetTimerbyFunctionName 0 "ExitDialogue" (Variables|/Script/Engine.SoundBase|GetDuration (Variables|/Game/SpookyGame/Blueprints/Dialogue/BP_VoiceLine.BP_VoiceLine_C|GetVoiceLine (Utilities|Array|Get(acopy) (Variables|/Game/SpookyGame/Blueprints/Dialogue/BP_Dialogue.BP_Dialogue_C|GetDialogue (Variables|Default|GetCurrentDialogue)) (- (Variables|Default|GetDialogueCurrentIndex) 1))))))
              (Variables|Default|SetDialogueExitTimerHandle _returnvalue_2))))))))

(fn SetDialogue
  (params (Dialogue :type BP%20Dialogue%20Object%20Reference))
  (Variables|Default|SetCurrentDialogue Dialogue))

(fn SkipVoiceLine
  (bind _dialoguetimerhandle (Variables|Default|GetDialogueTimerHandle))
  (if (Utilities|Time|IsTimerActivebyHandle _dialoguetimerhandle)
    (Utilities|Time|ClearandInvalidateTimerbyHandle _dialoguetimerhandle)
    (CallFunction|StartDialogue)
    (else
      (CallFunction|ExitDialogue))))

(fn ExitDialogue
  (bind _dialogueexittimerhandle (Variables|Default|GetDialogueExitTimerHandle))
  (bind _dialoguetimerhandle (Variables|Default|GetDialogueTimerHandle))
  (Utilities|FlowControl|Sequence
    (:then_0
      (if (Utilities|Time|IsTimerActivebyHandle _dialogueexittimerhandle)
        (Utilities|Time|ClearandInvalidateTimerbyHandle _dialogueexittimerhandle)))
    (:then_1
      (if (Utilities|Time|IsTimerActivebyHandle _dialoguetimerhandle)
        (Utilities|Time|ClearandInvalidateTimerbyHandle _dialoguetimerhandle)))
    (:then_2
      (Audio|Components|Audio|Stop (Variables|Default|GetAudio))
      (Variables|Default|SetIsDialogueActive false)
      (CallFunction|UnlockPlayer)
      (Variables|Default|SetDialogueCurrentIndex 0))
    (:then_3
      (Default|AddDialogue (Variables|Default|GetBP_NarrativeLog) (Variables|Default|GetCurrentDialogue)))
    (:then_4
      (Pawn|Possess (Game|GetPlayerController 0) (Variables|Default|GetPlayer)))))