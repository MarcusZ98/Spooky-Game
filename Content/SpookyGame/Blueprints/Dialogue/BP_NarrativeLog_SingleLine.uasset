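; Possessable narrative log that replays collected dialogue voice lines, which other code adds uniquely through AddDialogue.
; On possession it plays an enter sound and starts at the newest line, or returns control to BP_SG_Player if empty.
; PlayLine plays a 2D voice line under an audio focus event and sets a duration-based timer to advance.
; Up/Down keys step through lines with limit feedback, while Enter stops playback and repossesses the player.
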(event Custom|LimitReached
  ;[1 1 1] ChangeLine
  (Audio|PlaySound2D (Variables|Default|GetCannotSelectSound) 1.0 1.0 0.0 0 0))

(event Custom|Play%20Line
  (bind _currentindex (Variables|Default|GetCurrentIndex))
  (bind _voicelines (Variables|Default|GetVoiceLines))
  (bind _output (Utilities|Array|Get(acopy) _voicelines _currentindex))
  (bind _voiceline (Variables|/Game/SpookyGame/Blueprints/Dialogue/BP_VoiceLine.BP_VoiceLine_C|GetVoiceLine _output))
  ;[1 1 1] PlayLine
  (Utilities|IsValid (Variables|Default|GetCurrentAC)
    (:Is%20Valid
      (Audio|Components|Audio|Stop (Variables|Default|GetCurrentAC)))
    (:Is%20Not%20Valid
      _))
  (if (Utilities|Array|IsValidIndex (Variables|Default|GetVoiceLines) (Variables|Default|GetCurrentIndex))
    (CallFunction|BeginFocusEvent _voiceline true 0.1 0.0 (Utilities|Struct|MakeSTR_MapWrapper (Variables|Default|GetCustom%20Override%20Sound%20and%20Volume%20Map)))
    (bind _returnvalue (Audio|SpawnSound2D _voiceline 1.0 1.0 0.0 0))
    (Variables|Default|SetCurrentAC _returnvalue)
    (Development|PrintString (Utilities|String|ToString(Integer) (Variables|Default|GetCurrentIndex)))
    (bind _returnvalue_2 (Utilities|Time|SetTimerbyEvent (delegate Custom|Play%20Line) (+ (Variables|/Script/Engine.SoundBase|GetDuration _voiceline) (Variables|Default|GetTimeBetweenVoiceLines)) true))
    (Variables|Default|SetVLTimerHandle _returnvalue_2)
    (Math|Integer|IncrementInt (Variables|Default|GetCurrentIndex))))

(event EventBeginPlay
  ;[1 1 1] Begin
  (bind _returnvalue (Actor|GetActorOfClass "/Game/SpookyGame/Blueprints/Player/BP_SG_Player.BP_SG_Player_C"))
  (Variables|Default|SetPlayer%20REF _returnvalue))

(event EventPossessed
  (params (NewController :type Controller%20Object%20Reference))
  (bind _enterlog (Variables|Default|GetEnterLog))
  ;[1 1 1] OnPosses
  (if (Utilities|Array|IsNotEmpty (Variables|Default|GetVoiceLines))
    (Audio|PlaySound2D _enterlog 1.0 1.0 0.0 0 0)
    (Utilities|FlowControl|Delay (Variables|/Script/Engine.SoundBase|GetDuration _enterlog))
    (Variables|Default|SetCurrentIndex (Utilities|Array|LastIndex (Variables|Default|GetVoiceLines)))
    (CallFunction|PlayLine)
    (else
      (Development|PrintString "No Dialogue")
      (Utilities|FlowControl|DelayUntilNextTick)
      (Pawn|Possess (Game|GetPlayerController 0) (Variables|Default|GetPlayer%20REF)))))

(event Input|KeyboardEvents|Enter
  (params (Key :type Key%20Structure :default "None"))
  ;[1 1 1] ExitLog
  (:Pressed
    (Variables|Default|SetCurrentIndex -1)
    (Pawn|Possess (Game|GetPlayerController 0) (Variables|Default|GetPlayer%20REF))
    (CallFunction|ExitFocusEvent 1.0)
    (Audio|Components|Audio|Stop (Variables|Default|GetCurrentAC))
    (Audio|PlaySound2D (Variables|Default|GetExitLog) 1.0 1.0 0.0 0 0)))

(event Input|KeyboardEvents|Down
  (params (Key :type Key%20Structure :default "None"))
  ;[1 1 1] ChangeLine
  (:Pressed
    (if (<= (Variables|Default|GetCurrentIndex) (Utilities|Array|LastIndex (Variables|Default|GetVoiceLines)))
      (Audio|PlaySound2D (Variables|Default|GetSelectSound) 1.0 1.0 0.0 0 0)
      (CallFunction|PlayLine)
      (else
        (CallFunction|LimitReached)))))

(event Input|KeyboardEvents|Up
  (params (Key :type Key%20Structure :default "None"))
  ;[1 1 1] ChangeLine
  (:Pressed
    (if (== (Variables|Default|GetCurrentIndex) 1)
      (CallFunction|LimitReached)
      (else
        (Audio|PlaySound2D (Variables|Default|GetSelectSound) 1.0 1.0 0.0 0 0)
        (Variables|Default|SetCurrentIndex (- (Variables|Default|GetCurrentIndex) 2))
        (CallFunction|PlayLine)))))

(fn ConstructionScript)

(fn AddDialogue
  (params (Dialogue :type BP%20Dialogue%20Object%20Reference))
  (bind _newparam (CallFunction|AddLines Dialogue))
  (return _newparam))

(fn AddLines
  (params (Dialogue :type BP%20Dialogue%20Object%20Reference))
  (for _array_element (Variables|/Game/SpookyGame/Blueprints/Dialogue/BP_Dialogue.BP_Dialogue_C|GetDialogue Dialogue)
    (bind _returnvalue (Utilities|Array|AddUnique (Variables|Default|GetVoiceLines) _array_element))
    (LocalVariables|SetUnique _returnvalue))
  (return (LocalVariables|GetUnique)))

(fn HasLines
  (return (Utilities|Array|IsNotEmpty (Variables|Default|GetVoiceLines))))