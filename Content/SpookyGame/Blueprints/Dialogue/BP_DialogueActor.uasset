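; BP_DialogueActor plays a sequence of positioned dialogue sounds, starting on BeginPlay.
; AddVoiceLines builds a BP_DialogueLine for each SoundFileNames entry, pairing it with the matching SoundPositions entry.
; PlayDialogueEvent spawns a sound at its line's location, and its audio-finished callback increments I and repeats until past the last index.
; PlayLine always receives index 0, so every pass replays the first line rather than line I.
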(event OnAudioFinished(Audio))

(event Custom|Play%20Dialogue%20Event
  ;[1 1 1] IndexingCheck
  (if (<= (Variables|Default|Geti) (Utilities|Array|LastIndex (Variables|Default|GetVoiceLines)))
    (bind _audio_component (CallFunction|PlayLine))
    (EventDispatchers|BindEventtoOnAudioFinished _audio_component (delegate Custom|Finish))))

(event Custom|Finish
  (Math|Integer|IncrementInt (Variables|Default|Geti)
    (:%20%20
      (CallFunction|PlayDialogueEvent))))

(event EventBeginPlay
  (CallFunction|AddVoiceLines)
  (CallFunction|PlayDialogueEvent))

(fn ConstructionScript)

(fn AddVoiceLines
  (for (_array_element _array_index) (Variables|Default|GetSoundFileNames)
    (bind _returnvalue (Game|AddComponentbyClass "/Game/SpookyGame/Blueprints/Dialogue/BP_DialogueLine.BP_DialogueLine_C"))
    (Utilities|Array|Add (Variables|Default|GetVoiceLines) _returnvalue)
    (Default|SetValues _returnvalue _array_element (Utilities|Array|Get(acopy) (Variables|Default|GetSoundPositions) _array_index))))

(fn PlayLine
  (params (Index :type Integer))
  (bind _voicelines (Variables|Default|GetVoiceLines))
  (bind _output (Utilities|Array|Get(acopy) _voicelines Index))
  (bind _returnvalue (Audio|SpawnSoundatLocation (Variables|/Game/SpookyGame/Blueprints/Dialogue/BP_DialogueLine.BP_DialogueLine_C|GetCue _output) (Variables|/Game/SpookyGame/Blueprints/Dialogue/BP_DialogueLine.BP_DialogueLine_C|GetPosition _output) "0, 0, 0" 1.0 1.0 0.0 0 0))
  (return _returnvalue))