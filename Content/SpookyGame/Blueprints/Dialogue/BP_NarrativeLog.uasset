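; Possessable narrative log that replays the most recently added dialogue through BP_DialogueManager.
; AddDialogue stores unique entries, and on possession the last one is set on the manager and started.
; Space skips the current voice line, while Enter exits the dialogue and hands possession back to the BP_SG_Player found at BeginPlay.
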(event EventBeginPlay
  (bind _returnvalue (Actor|GetActorOfClass "/Game/SpookyGame/Blueprints/Dialogue/BP_DialogueManager.BP_DialogueManager_C"))
  (Variables|Default|SetDM _returnvalue)
  (bind _returnvalue_2 (Actor|GetActorOfClass "/Game/SpookyGame/Blueprints/Player/BP_SG_Player.BP_SG_Player_C"))
  (Variables|Default|SetPlayer%20REF _returnvalue_2))

(event Collision|EventActorBeginOverlap
  (params (OtherActor :type Actor%20Object%20Reference)))

(event EventTick
  (params (DeltaSeconds :type Float%20%28single-precision%29)))

(event EventPossessed
  (params (NewController :type Controller%20Object%20Reference))
  (bind _dialogues (Variables|Default|GetDialogues))
  (bind _dm (Variables|Default|GetDM))
  (Utilities|IsValid _dm
    (:Is%20Valid
      (Default|SetDialogue _dm (Utilities|Array|Get(acopy) _dialogues (Utilities|Array|LastIndex _dialogues)))
      (Default|StartDialogue _dm))
    (:Is%20Not%20Valid
      (Development|PrintString "DM Variable is null"))))

(event Input|KeyboardEvents|S
  (params (Key :type Key%20Structure :default "None")))

(event Input|KeyboardEvents|W
  (params (Key :type Key%20Structure :default "None")))

(event Input|KeyboardEvents|Enter
  (params (Key :type Key%20Structure :default "None"))
  (:Pressed
    (Default|ExitDialogue (Variables|Default|GetDM))
    (Pawn|Possess (Game|GetPlayerController 0) (Variables|Default|GetPlayer%20REF))))

(event Input|KeyboardEvents|SpaceBar
  (params (Key :type Key%20Structure :default "None"))
  (:Pressed
    (Default|SkipVoiceLine (Variables|Default|GetDM))))

(fn ConstructionScript)

(fn AddDialogue
  (params (Dialogue :type BP%20Dialogue%20Object%20Reference))
  (Utilities|Array|AddUnique (Variables|Default|GetDialogues) Dialogue))