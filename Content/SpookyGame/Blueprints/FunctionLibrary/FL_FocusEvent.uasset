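; Blueprint function library that starts and ends audio focus events by changing sound class volumes on the SM_Base sound mix.
; BeginFocusEvent can fade sound classes to a shared volume, skipping the focused sound's class only if it also has a custom override.
; It then applies per-class volumes from the custom override map.
; ExitFocusEvent fades every listed class back to the default override volume.
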(fn BeginFocusEvent
  (params (SoundToFocusOn :type Sound%20Base%20Object%20Reference) (bAdjustAllOtherSound? :type Boolean) (New%20Volume :type Float%20%28double-precision%29) (FadeInTime :type Float%20%28double-precision%29) (Custom%20Override%20Sound%20and%20Volume :type STR%20Map%20Wrapper%20Structure))
  (if bAdjustAllOtherSound?
    (for _array_element (LocalVariables|GetAllSoundClasses)
      (if (or (!= (Variables|/Script/Engine.SoundBase|GetSoundClassObject SoundToFocusOn) _array_element) (not (Utilities|Map|Contains (.map Custom%20Override%20Sound%20and%20Volume) _array_element)))
        (Audio|SetSoundMixClassOverride 0 "/Game/SpookyGame/Blueprints/FrameWork/SM_Base.SM_Base" _array_element New%20Volume 1.0 FadeInTime true))))
  (bind _keys (Utilities|Map|Keys (.map Custom%20Override%20Sound%20and%20Volume)))
  (for _array_element_2 _keys
    (Audio|SetSoundMixClassOverride 0 "/Game/SpookyGame/Blueprints/FrameWork/SM_Base.SM_Base" _array_element_2 (.Value (Utilities|Map|Find (.map Custom%20Override%20Sound%20and%20Volume) _array_element_2)) 1.0 FadeInTime true)))

(fn ExitFocusEvent
  (params (Fade%20Out%20Time :type Float%20%28double-precision%29))
  (for _array_element (LocalVariables|GetAllSoundClasses)
    (Audio|SetSoundMixClassOverride 0 "/Game/SpookyGame/Blueprints/FrameWork/SM_Base.SM_Base" _array_element 1.0 1.0 Fade%20Out%20Time true)))