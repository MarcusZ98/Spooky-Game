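; Player dialogue component that handles input for skipping dialogue voice lines and opening the narrative log.
; On BeginPlay it finds and caches the dialogue manager and the single-line narrative log actor in the level.
; Space skips the current voice line through the manager while dialogue is active.
; Enter makes the player controller possess the narrative log if it has lines.
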(event EventBeginPlay
  (Utilities|FlowControl|Sequence
    (:then_0
      (bind _returnvalue (Actor|GetActorOfClass "/Game/SpookyGame/Blueprints/Dialogue/BP_DialogueManager.BP_DialogueManager_C"))
      (Variables|Default|SetDM _returnvalue))
    (:then_1
      (bind _returnvalue_2 (Actor|GetActorOfClass "/Game/SpookyGame/Blueprints/Dialogue/BP_NarrativeLog_SingleLine.BP_NarrativeLog_SingleLine_C"))
      (Variables|Default|SetNarrativeLog _returnvalue_2))))

(event Input|KeyboardEvents|SpaceBar
  (params (Key :type Key%20Structure :default "None"))
  (:Pressed
    (CallFunction|SkipLine)))

(event Input|KeyboardEvents|Enter
  (params (Key :type Key%20Structure :default "None"))
  (:Pressed
    (if (Default|HasLines (Variables|Default|GetNarrativeLog))
      (Pawn|Possess (Game|GetPlayerController 0) (Variables|Default|GetNarrativeLog)))))

(fn SkipLine
  (if (Variables|/Game/SpookyGame/Blueprints/Dialogue/BP_DialogueManager.BP_DialogueManager_C|GetIsDialogueActive (Variables|Default|GetDM))
    (Default|SkipVoiceLine (Variables|Default|GetDM))))