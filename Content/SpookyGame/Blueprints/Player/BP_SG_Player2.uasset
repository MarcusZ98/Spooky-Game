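; Player character for SpookyGame that handles interaction, movement sounds and receiving the teddy.
; An overlap sphere tracks the current BPI_Interactable object, which the interact input triggers with the player as sender.
; Capsule hits play speed-scaled bump and wall-slide sounds, gated by DoOnce nodes, with the bump re-armed when WallCheck leaves a non-interactable.
; Tick drives footstep audio from velocity, and ReciveTeddy sets HasTeddy with a sound.
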(event OnComponentBeginOverlap(Sphere)
  (params (OverlappedComponent :type Primitive%20Component%20Object%20Reference) (OtherActor :type Actor%20Object%20Reference) (OtherComp :type Primitive%20Component%20Object%20Reference) (OtherBodyIndex :type Integer) (bFromSweep :type Boolean) (SweepResult :type Hit%20Result%20Structure%20%28by%20ref%29))
  ;[1 1 1] Interact
  (if (Utilities|DoesObjectImplementInterface OtherActor "/Game/SpookyGame/Blueprints/Interfaces/BPI_Interactable.BPI_Interactable_C")
    (Variables|Default|SetCurrentInteractableObject OtherActor)
    (Audio|PlaySound2D "/Game/SpookyGame/Audio/All_Rooms/SFX/SFX_Interact_Active.SFX_Interact_Active" 1.0 1.0 0.0 0 0)))

(event OnComponentEndOverlap(Sphere)
  (params (OverlappedComponent :type Primitive%20Component%20Object%20Reference) (OtherActor :type Actor%20Object%20Reference) (OtherComp :type Primitive%20Component%20Object%20Reference) (OtherBodyIndex :type Integer))
  ;[1 1 1] Interact
  (if (== OtherActor (Variables|Default|GetCurrentInteractableObject))
    (Variables|Default|SetCurrentInteractableObject 0)))

(event OnComponentHit(CapsuleComponent)
  (params (HitComponent :type Primitive%20Component%20Object%20Reference) (OtherActor :type Actor%20Object%20Reference) (OtherComp :type Primitive%20Component%20Object%20Reference) (NormalImpulse :type Vector :default "0, 0, 0") (Hit :type Hit%20Result%20Structure%20%28by%20ref%29))
  (bind _returnvalue (Transformation|GetVelocity))
  (bind _returnvalue_2 (Math|Vector|VectorLength _returnvalue))
  (bind _returnvalue_3 (- _returnvalue_2 5e+01))
  (bind _returnvalue_4 (/ _returnvalue_3 4.5e+02))
  (bind _returnvalue_5 (+ _returnvalue_4 0.85))
  ;[1 1 1] Walking into object
  ;;[1 1 1] Check if moving
  (if (> _returnvalue_2 5e+01)
    (Utilities|FlowControl|Sequence
      (:then_0
        _)
      (:then_1
        (Utilities|FlowControl|DoOnce false :!label _label
          (:Completed
            (Audio|PlaySoundatLocation "/Game/SpookyGame/Audio/Player/SFX_Walk_Against_Wall_Cue.SFX_Walk_Against_Wall_Cue" (.impactpoint Hit) "0, 0, 0" _returnvalue_5 _returnvalue_5 0.0 0 0 0 0) ; Wall slide sound
            (Utilities|FlowControl|Delay 1.0)
            (goto _label Reset))))))
  (Utilities|FlowControl|DoOnce false
    (:Completed
      (Audio|PlaySoundatLocation "/Game/SpookyGame/Audio/Player/Kick/SFX_Kick_Cue.SFX_Kick_Cue" (.impactpoint Hit) "0, 0, 0" (- 1.0 (/ _returnvalue_2 2e+02)) (+ (/ _returnvalue_2 333.0) 1.0) 0.0 0 0 0 0) ; Bump wall sound
    )))

(event OnComponentEndOverlap(WallCheck)
  (params (OverlappedComponent :type Primitive%20Component%20Object%20Reference) (OtherActor :type Actor%20Object%20Reference) (OtherComp :type Primitive%20Component%20Object%20Reference) (OtherBodyIndex :type Integer))
  ;[1 1 1] If Wallcheck no longer overlaps with wall
  (if (not (Utilities|DoesObjectImplementInterface OtherActor "/Game/SpookyGame/Blueprints/Interfaces/BPI_Interactable.BPI_Interactable_C"))
    (CallFunction|MovedAwayfromWall)))

(event OnComponentBeginOverlap(WallCheck)
  (params (OverlappedComponent :type Primitive%20Component%20Object%20Reference) (OtherActor :type Actor%20Object%20Reference) (OtherComp :type Primitive%20Component%20Object%20Reference) (OtherBodyIndex :type Integer) (bFromSweep :type Boolean) (SweepResult :type Hit%20Result%20Structure%20%28by%20ref%29))
  ;[1 1 1] Debugging Wallcheck overlap
)

(event Custom|Moved%20Away%20From%20Wall
  (bind _returnvalue (Transformation|GetVelocity))
  (bind _returnvalue_2 (Math|Vector|VectorLength _returnvalue))
  ;[1 1 1] Walking into object
  (Utilities|FlowControl|DoOnce false) ; enters at Reset
)

(event Input|EnhancedActionEvents|EnhancedInputActionIA_Interact
  (params (ActionValue :type Boolean) (ElapsedSeconds :type Float%20%28double-precision%29) (TriggeredSeconds :type Float%20%28double-precision%29) (InputAction :type Input%20Action%20Object%20Reference :default "/Game/ThirdPerson/Input/Actions/IA_Interact.IA_Interact"))
  ;[1 1 1] Interact
  (:Started
    (Class|BPIInteractable|TriggerEvent(Message) (Variables|Default|GetCurrentInteractableObject) self)))

(event EventTick
  (params (DeltaSeconds :type Float%20%28single-precision%29))
  ;[1 1 1] WalkingLogic
  (if (> (Math|Vector|VectorLength (Transformation|GetVelocity)) 75.0)
    (if (not (Audio|Components|Audio|IsPlaying (Variables|Default|GetWalkAudio)))
      (Utilities|FlowControl|DoOnce false :!label _label
        (:Completed
          (Audio|Components|Audio|Play (Variables|Default|GetWalkAudio) 0.0)
          (Utilities|FlowControl|Delay (Math|Random|RandomFloatinRange 0.75 1.0))
          (goto _label Reset))))
    (else
      (Audio|Components|Audio|Stop (Variables|Default|GetWalkAudio)))))

(event EventBeginPlay)

(event EventUnpossessed
  (params (OldController :type Controller%20Object%20Reference))
  (Variables|/Script/Engine.MovementComponent|SetVelocity (Variables|Character|GetCharacterMovement) "0, 0, 0"))

(fn ConstructionScript)

(fn ReciveTeddy
  (Audio|PlaySound2D (Variables|Audio|GetAudio_ReciveTeddy) 1.0 1.0 0.0 0 0)
  (Variables|Default|SetbHasTeddy? true)
  (Development|PrintString "Player have teddy now"))