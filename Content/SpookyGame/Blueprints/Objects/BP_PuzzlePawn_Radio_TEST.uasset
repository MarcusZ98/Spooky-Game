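; Test version of a radio puzzle pawn with two tuning knobs, each searching for its own target band by sound.
; Input actions step each knob's value within limits, playing a turn sound or a ping when blocked.
; Tick maps each value to far static, near static or on-target audio, using DoOnce gates to switch loops only on zone changes and raising another layer's volume on target.
; Older held-key knob logic remains disconnected.
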(event Input|EnhancedActionEvents|EnhancedInputActionIA_Radio_Right
  (params (ActionValue :type Float%20%28double-precision%29) (ElapsedSeconds :type Float%20%28double-precision%29) (TriggeredSeconds :type Float%20%28double-precision%29) (InputAction :type Input%20Action%20Object%20Reference :default "/Game/ThirdPerson/Input/Actions/IA_Radio_Right.IA_Radio_Right"))
  (bind _right_audio (Variables|Default|GetRight_Audio))
  (bind _returnvalue (Transformation|GetWorldLocation _right_audio))
  (:Started
    (if (Math|Float|InRange(Float) (+ (Variables|Default|GetRight_Value) (* ActionValue (Variables|Default|GetValue%20Increase))) 0.0 1.8e+02)
      (Variables|Default|SetRight_Value (+ (Variables|Default|GetRight_Value) (* ActionValue (Variables|Default|GetValue%20Increase))))
      (Audio|PlaySoundatLocation "/Game/SpookyGame/Audio/Captain/SFX/SFX_Knob_Turn_Loop.SFX_Knob_Turn_Loop" _returnvalue "0, 0, 0" 1.0 1.0 0.0 0 0 0 0)
      (else
        (Audio|PlaySoundatLocation "/Engine/EngineSounds/1kSineTonePing.1kSineTonePing" _returnvalue "0, 0, 0" 1.0 1.0 0.0 0 0 0 0)))))

(event Input|EnhancedActionEvents|EnhancedInputActionIA_Radio_Left
  (params (ActionValue :type Float%20%28double-precision%29) (ElapsedSeconds :type Float%20%28double-precision%29) (TriggeredSeconds :type Float%20%28double-precision%29) (InputAction :type Input%20Action%20Object%20Reference :default "/Game/ThirdPerson/Input/Actions/IA_Radio_Left.IA_Radio_Left"))
  (bind _left_audio (Variables|Default|GetLeft_Audio))
  (bind _returnvalue (Transformation|GetWorldLocation _left_audio))
  (:Started
    (if (Math|Float|InRange(Float) (+ (Variables|Default|GetLeft_Value) (* ActionValue (Variables|Default|GetValue%20Increase))) 0.0 1.8e+02)
      (Variables|Default|SetLeft_Value (+ (Variables|Default|GetLeft_Value) (* ActionValue (Variables|Default|GetValue%20Increase))))
      (Audio|PlaySoundatLocation "/Game/SpookyGame/Audio/Captain/SFX/SFX_Knob_Turn_Loop.SFX_Knob_Turn_Loop" _returnvalue "0, 0, 0" 1.0 1.0 0.0 0 0 0 0)
      (else
        (Audio|PlaySoundatLocation "/Engine/EngineSounds/1kSineTonePing.1kSineTonePing" _returnvalue "0, 0, 0" 1.0 1.0 0.0 0 0 0 0)))))

(event EventBeginPlay
  (|CallParentFunction))

(event Collision|EventActorBeginOverlap
  (params (OtherActor :type Actor%20Object%20Reference)))

(event EventTriggerEvent
  (params (PlayerREF :type BP%20SG%20Player%20Object%20Reference))
  (|CallParentFunction PlayerREF)
  (Audio|Components|Audio|Stop (Variables|Default|GetEnvironmentalAudio))
  (Development|PrintString "STOP PLAY"))

(event EventTick
  (params (DeltaSeconds :type Float%20%28single-precision%29))
  (bind _right_audio2 (Variables|Default|GetRight_Audio2))
  (bind _left_audio2 (Variables|Default|GetLeft_Audio2))
  (bind _left_audio3 (Variables|Default|GetLeft_Audio3))
  (bind _left_value (Variables|Default|GetLeft_Value))
  (bind _right_audio3 (Variables|Default|GetRight_Audio3))
  (bind _right_value (Variables|Default|GetRight_Value))
  (Utilities|FlowControl|Sequence
    (:then_0
      (if (not (== (Variables|Default|GetLeft_Value) 9e+01))
        (if (Math|Float|InRange(Float) (Variables|Default|GetLeft_Value) 38.0 48.0)
          (Utilities|FlowControl|Sequence
            (:then_0
              (Utilities|FlowControl|DoOnce false :!label _label
                (:Completed
                  (Utilities|FlowControl|Sequence
                    (:then_0
                      (Audio|Components|Audio|SetSound _left_audio2 "/Game/SpookyGame/Audio/Captain/UI/UI_Radio_Journal_Noise_Loop.UI_Radio_Journal_Noise_Loop")
                      (Audio|Components|Audio|Play _left_audio2 0.0 :!label _label_2))
                    (:then_1
                      (goto _label_5 Reset))
                    (:then_2
                      (goto _label_3 Reset))))))
            (:then_1
              (Audio|Components|Audio|SetVolumeMultiplier _left_audio3 0.5 :!class /Script/Engine.AudioComponent)))
          (elif (Math|Float|InRange(Float) (Variables|Default|GetLeft_Value) 23.0 63.0)
            (Utilities|FlowControl|DoOnce false :!label _label_3
              (:Completed
                (Utilities|FlowControl|Sequence
                  (:then_0
                    (Audio|Components|Audio|SetSound _left_audio2 "/Game/SpookyGame/Audio/Captain/SFX/SFX_Radio_Static_Loop_02.SFX_Radio_Static_Loop_02")
                    (goto _label_2))
                  (:then_1
                    (goto _label_5 Reset))
                  (:then_2
                    (goto _label Reset))
                  (:then_3
                    (Audio|Components|Audio|SetVolumeMultiplier _left_audio3 0.01 :!class /Script/Engine.AudioComponent :!label _label_4)))))
            (elif (or (< _left_value 23.0) (> _left_value 63.0))
              (Utilities|FlowControl|DoOnce false :!label _label_5
                (:Completed
                  (Utilities|FlowControl|Sequence
                    (:then_0
                      (Audio|Components|Audio|SetSound _left_audio2 "/Game/SpookyGame/Audio/Captain/SFX/SFX_Radio_Static_Loop_01.SFX_Radio_Static_Loop_01")
                      (goto _label_2))
                    (:then_1
                      (goto _label Reset))
                    (:then_2
                      (goto _label_3 Reset))
                    (:then_3
                      (goto _label_4))))))))))
    (:then_1
      (if (not (== (Variables|Default|GetRight_Value) 9e+01))
        (if (Math|Float|InRange(Float) (Variables|Default|GetRight_Value) 116.0 126.0)
          (Utilities|FlowControl|Sequence
            (:then_0
              (Utilities|FlowControl|DoOnce false :!label _label_6
                (:Completed
                  (Utilities|FlowControl|Sequence
                    (:then_0
                      (Audio|Components|Audio|SetSound _right_audio2 "/Game/SpookyGame/Audio/Captain/UI/UI_Radio_Journal_Noise_Loop.UI_Radio_Journal_Noise_Loop")
                      (Audio|Components|Audio|SetVolumeMultiplier _right_audio2 1.0 :!class /Script/Engine.AudioComponent)
                      (Audio|Components|Audio|Play _right_audio2 0.0 :!label _label_7))
                    (:then_1
                      (goto _label_11 Reset))
                    (:then_2
                      (goto _label_8 Reset))))))
            (:then_1
              (Audio|Components|Audio|SetVolumeMultiplier _right_audio3 0.5 :!class /Script/Engine.AudioComponent)))
          (elif (Math|Float|InRange(Float) (Variables|Default|GetRight_Value) 101.0 141.0)
            (Utilities|FlowControl|DoOnce false :!label _label_8
              (:Completed
                (Utilities|FlowControl|Sequence
                  (:then_0
                    (Audio|Components|Audio|SetSound _right_audio2 "/Game/SpookyGame/Audio/Captain/SFX/SFX_Radio_Static_Loop_02.SFX_Radio_Static_Loop_02")
                    (Audio|Components|Audio|SetVolumeMultiplier _right_audio2 0.5 :!class /Script/Engine.AudioComponent :!label _label_9)
                    (goto _label_7))
                  (:then_1
                    (goto _label_11 Reset))
                  (:then_2
                    (goto _label_6 Reset))
                  (:then_3
                    (Audio|Components|Audio|SetVolumeMultiplier _right_audio3 0.01 :!class /Script/Engine.AudioComponent :!label _label_10)))))
            (elif (or (< _right_value 101.0) (> _right_value 141.0))
              (Utilities|FlowControl|DoOnce false :!label _label_11
                (:Completed
                  (Utilities|FlowControl|Sequence
                    (:then_0
                      (Audio|Components|Audio|SetSound _right_audio2 "/Game/SpookyGame/Audio/Captain/SFX/SFX_Radio_Static_Loop_01.SFX_Radio_Static_Loop_01")
                      (goto _label_9))
                    (:then_1
                      (goto _label_6 Reset))
                    (:then_2
                      (goto _label_8 Reset))
                    (:then_3
                      (goto _label_10))))))))))))

(event Input|KeyboardEvents|Right
  (params (Key :type Key%20Structure :default "None"))
  ;[1 0 0] Legacy
)

(event Input|KeyboardEvents|A
  (params (Key :type Key%20Structure :default "None"))
  ;[1 0 0] Legacy
)

(event Input|KeyboardEvents|D
  (params (Key :type Key%20Structure :default "None"))
  ;[1 0 0] Legacy
)

(event Input|KeyboardEvents|Left
  (params (Key :type Key%20Structure :default "None"))
  ;[1 0 0] Legacy
)

(fn ConstructionScript
  (|CallParentFunction))