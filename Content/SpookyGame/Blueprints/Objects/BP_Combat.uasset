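; BP_Combat is a possessed audio-cue combat minigame where the player counters enemy attacks from the left, center or right.
; A random positional attack sound sets the correct answer, and WASD-style or arrow keys (left, up, right) allow one counter per round.
; Hits count toward victory and misses cost health, with timers starting new rounds.
; Defeat reloads the level; victory plays a sound, repossesses the game state's player and destroys the actor.
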(event Custom|ExitCombat
  ;[1 1 1] Exit Combat
  (Pawn|Possess (Game|GetPlayerController 0) (Game|GetPlayerCharacter 0)))

(event Custom|Play%20Enemy%20Attack%20Sound
  (params (Index :type Integer))
  (Audio|Components|Audio|Play (Utilities|Array|Get(acopy) (Variables|Default|GetAudioAttackArray) Index) 0.0))

(event EventBeginPlay
  ;[1 1 1] Intro combat
  (Utilities|FlowControl|Delay 3.0)
  (Variables|Default|SetAudioAttackArray (Utilities|Array|MakeArray (Variables|Default|GetRightAudio) (Variables|Default|GetCenterAudio) (Variables|Default|GetLeftAudio)))
  (Variables|Default|SetAudioCounterArray (Utilities|Array|MakeArray (Variables|Default|GetRightAudioPC) (Variables|Default|GetCenterAudioPC) (Variables|Default|GetLeftAudioPC)))
  (bind _index (CallFunction|GetRandomIndex))
  (CallFunction|PlayEnemyAttackSound _index)
  (Variables|Default|SetbCounterAttack true))

(event Input|KeyboardEvents|Up
  (params (Key :type Key%20Structure :default "None"))
  (:Pressed
    (CallFunction|CounterAttack 1)))

(event Input|KeyboardEvents|W
  (params (Key :type Key%20Structure :default "None"))
  (:Pressed
    (CallFunction|CounterAttack 1)))

(event Input|KeyboardEvents|D
  (params (Key :type Key%20Structure :default "None"))
  (:Pressed
    (CallFunction|CounterAttack)))

(event Input|KeyboardEvents|Right
  (params (Key :type Key%20Structure :default "None"))
  (:Pressed
    (CallFunction|CounterAttack)))

(event Input|KeyboardEvents|A
  (params (Key :type Key%20Structure :default "None"))
  (:Pressed
    (CallFunction|CounterAttack 2)))

(event Input|KeyboardEvents|Left
  (params (Key :type Key%20Structure :default "None"))
  (:Pressed
    (CallFunction|CounterAttack 2)))

(fn ConstructionScript)

(fn GetRandomIndex
  (bind _output_get (Variables|Default|SetCurrentIndex (.OutIndex (Utilities|Array|Random (Variables|Default|GetAudioAttackArray)))))
  (return _output_get))

(fn CounterAttack
  (params (Index :type Integer))
  (LocalVariables|SetCounterIndex Index)
  (if (Variables|Default|GetbCounterAttack)
    (Audio|Components|Audio|Play (Utilities|Array|Get(acopy) (Variables|Default|GetAudioCounterArray) Index) 0.0)
    (Variables|Default|SetbCounterAttack false)
    (if (== (LocalVariables|GetCounterIndex) (Variables|Default|GetCurrentIndex))
      (CallFunction|HitEnemy)
      (else
        (CallFunction|MissEnemy)))))

(fn StartCombat
  (bind _index (CallFunction|GetRandomIndex))
  (CallFunction|PlayEnemyAttackSound _index)
  (Variables|Default|SetbCounterAttack true))

(fn HitEnemy
  (bind _currentenemiesdefeated (Variables|Default|GetCurrentEnemiesDefeated))
  (Math|Integer|IncrementInt _currentenemiesdefeated
    (:%20%20
      (if (== _currentenemiesdefeated (Variables|Default|GetEnemiesToDefeat))
        (CallFunction|EndCombat)
        (else
          (Development|PrintString "EnemyHit")
          (Utilities|Time|SetTimerbyFunctionName 0 "StartCombat" 4.0))))))

(fn MissEnemy
  (Math|Integer|DecrementInt (Variables|Default|GetHealth)
    (:%20%20
      (Development|PrintString "Missed Enemy")
      (if (== (Variables|Default|GetHealth) 0)
        (bind _returnvalue (Game|GetCurrentLevelName true))
        (Game|OpenLevel(byName) (Utilities|String|StringToName _returnvalue))
        (else
          (Utilities|Time|SetTimerbyFunctionName 0 "StartCombat" 4.0))))))

(fn EndCombat
  (bind _returnvalue (Audio|SpawnSoundatLocation "/Game/SpookyGame/Audio/Player/Player_Victory_Cue.Player_Victory_Cue" "0, 0, 0" "0, 0, 0" 1.0 1.0 0.0 0 0))
  (Utilities|Time|SetTimerbyFunctionName 0 "ReturnToPlayer" (Variables|/Script/Engine.SoundBase|GetDuration (Variables|/Script/Engine.AudioComponent|GetSound _returnvalue))))

(fn ReturntoPlayer
  (bind _asbp_sg_game_state (Utilities|Casting|CastToBP_SG_GameState (Game|GetGameState)))
  (Pawn|Possess (Game|GetPlayerController 0) (Variables|/Game/SpookyGame/Blueprints/FrameWork/BP_SG_GameState.BP_SG_GameState_C|GetBP_Player _asbp_sg_game_state))
  (Actor|DestroyActor))