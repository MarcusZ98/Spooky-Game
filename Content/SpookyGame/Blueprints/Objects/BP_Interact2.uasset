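; BP_Interact2 is an interactable object that plays a sound at its location when the Interact event fires while the player is in range.
; A Box overlap with BP_ThirdPersonCharacter toggles CanInteract and prints debug strings, with a 2D cue sound on entry.
; A SoundPlaying flag and fixed Delay block retriggering for a few seconds, independent of the sound's actual length.
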(event OnComponentBeginOverlap(Box)
  (params (OverlappedComponent :type Primitive%20Component%20Object%20Reference) (OtherActor :type Actor%20Object%20Reference) (OtherComp :type Primitive%20Component%20Object%20Reference) (OtherBodyIndex :type Integer) (bFromSweep :type Boolean) (SweepResult :type Hit%20Result%20Structure%20%28by%20ref%29))
  (Utilities|Casting|CastToBP_ThirdPersonCharacter OtherActor)
  (Variables|Default|SetCanInteract? true)
  (Audio|PlaySound2D "/Game/SpookyGame/Audio/SFX/SFX_Interact_Active.SFX_Interact_Active" 1.0 1.0 0.0 0 0)
  (Development|PrintString "caninteract SET TRUE"))

(event OnComponentEndOverlap(Box)
  (params (OverlappedComponent :type Primitive%20Component%20Object%20Reference) (OtherActor :type Actor%20Object%20Reference) (OtherComp :type Primitive%20Component%20Object%20Reference) (OtherBodyIndex :type Integer))
  (Utilities|Casting|CastToBP_ThirdPersonCharacter OtherActor)
  (Variables|Default|SetCanInteract? false)
  (Development|PrintString "INTERACT FALSE"))

(event Custom|Interact
  (if (not (Variables|Default|GetSound%20playing))
    (if (Variables|Default|GetCanInteract?)
      (Audio|PlaySoundatLocation (Variables|Default|GetInteractSound) (Transformation|GetActorLocation self) "0, 0, 0" 1.0 1.0 0.0 0 0 0 0)
      (Variables|Default|SetSound%20playing true)
      (Utilities|FlowControl|Delay 5.0)
      (Variables|Default|SetSound%20playing false))))

(fn ConstructionScript)