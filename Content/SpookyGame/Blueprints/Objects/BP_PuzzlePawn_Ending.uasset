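; BP_PuzzlePawn_Ending is the puzzle pawn for the game's ending, triggered when the player destroys the artifact.
; It starts a cellar ambient loop on BeginPlay, and TriggerEvent logs the artifact's destruction through SG_GameInstance.
; The LowerSound timeline then drives the volume of the environmental audio and cellar loop, disabling player input on every update.
; Input is never re-enabled here, as the EnableInput node is unconnected.
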(event EventBeginPlay
  (|CallParentFunction)
  (Audio|Components|Audio|Play (Variables|Default|GetSFX_Cellar_Ambient_Loop) 0.0))

(event EventTriggerEvent
  (params (PlayerREF :type BP%20SG%20Player%20Object%20Reference))
  (|CallParentFunction PlayerREF)
  (bind _assg_game_instance (Utilities|Casting|CastToSG_GameInstance (Game|GetGameInstance)))
  (Class|SGGameInstance|WritetoFile _assg_game_instance "Player destroyed artifact")
  (bind _volume_over_time (Timeline|Lower%20sound Play)
    (:Update
      (Utilities|FlowControl|Sequence
        (:then_0
          (Audio|Components|Audio|SetVolumeMultiplier (Variables|Default|GetEnvironmentalAudio) _volume_over_time :!class /Script/Engine.AudioComponent))
        (:then_1
          (Audio|Components|Audio|SetVolumeMultiplier (Variables|Default|GetSFX_Cellar_Ambient_Loop) _volume_over_time :!class /Script/Engine.AudioComponent))
        (:then_2
          (Input|DisableInput (Game|GetPlayerController 0)))))))

(fn ConstructionScript
  (|CallParentFunction))