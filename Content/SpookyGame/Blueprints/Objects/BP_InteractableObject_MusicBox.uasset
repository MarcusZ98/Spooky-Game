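; Interactable music box for a piano puzzle that plays the song of correct notes when the player triggers it.
; Unless the linked Piano is solved, it disables player movement, stops its environmental audio and plays the song.
; A linked Baby laughs halfway through; at the end movement returns and the interaction is recorded, while a flag blocks retriggering during playback.
; Stopplaying silences the audio and destroys the actor.
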(event Custom|Stop%20playing
  ;[1 1 1] Stop playing
  (Audio|Components|Audio|Stop (Variables|Default|GetEnvironmentalAudio))
  (Actor|DestroyActor))

(event EventTriggerEvent
  (params (PlayerREF :type BP%20SG%20Player%20Object%20Reference))
  (bind _musicboxsong (Variables|Default|GetMusicBoxSong))
  (bind _duration (Variables|/Script/Engine.SoundBase|GetDuration _musicboxsong))
  (bind _returnvalue (/ _duration 2.0))
  ;[1 1 1] Check against spamming
  (if (not (Variables|Default|GetIsPlayerInteracting))
    (Variables|Default|SetIsPlayerInteracting true)
    (if (Variables|/Game/SpookyGame/Blueprints/Objects/BP_PuzzlePawn.BP_PuzzlePawn_C|GetIsPuzzleCompleted (Variables|Default|GetPiano))
      (Development|PrintString "Puzzle is already completed")
      (else
        ;[1 1 1] Disable movement
        (Pawn|Components|CharacterMovement|DisableMovement (Variables|/Script/Engine.Character|GetCharacterMovement PlayerREF))
        ;[1 1 1] Pause enviromental sound
        (Audio|Components|Audio|Stop (Variables|Default|GetEnvironmentalAudio))
        ;[1 1 1] Play Right notes
        (Audio|PlaySoundatLocation _musicboxsong (Transformation|GetActorLocation) "0, 0, 0" 1.0 1.0 0.0 0 0 0 0)
        (bind _baby (Variables|Default|GetBaby)
          (:then
            (Utilities|FlowControl|Delay _returnvalue)
            ;[1 1 1] Make baby laugh
            (Default|BabyLaugh _baby _returnvalue)
            (Utilities|FlowControl|Delay _returnvalue)
            ;[1 1 1] Enable movement
            (Pawn|Components|CharacterMovement|SetMovementMode (Variables|/Script/Engine.Character|GetCharacterMovement PlayerREF) "MOVE_Walking" 0)
            (Variables|Default|SetIsPlayerInteracting false)
            (Variables|Default|SetPlayerHasInteractedWithMusicBox true))
          (:else
            (Development|PrintString "No baby attached" true true "(R=0.000000,G=0.660000,B=1.000000,A=1.000000)" 5.0)))))))

(fn ConstructionScript
  (|CallParentFunction))