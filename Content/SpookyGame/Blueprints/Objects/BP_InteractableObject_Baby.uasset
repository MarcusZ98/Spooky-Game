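; Interactable crying-baby object that responds to the player cradling it or bringing a teddy, which opens the door to the next level.
; Without the teddy, interaction branches on piano puzzle completion, playing timed cradle and laughter sounds.
; While unsolved, the laugh also briefly opens the cabinet, followed by April's one-time spoken hint about it.
; Separate events swap environmental crying for laughter during music-box playback or for looping cooing.
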(event Custom|Baby%20Laugh
  (params (MusicBoxDuration :type Float%20%28double-precision%29))
  (bind _laughingbaby (Variables|Default|GetLaughingBaby))
  ;[1 1 1] Baby Laugh
  (Audio|Components|Audio|Stop (Variables|Default|GetEnvironmentalAudio))
  (Audio|Components|Audio|Play _laughingbaby 0.0)
  (Utilities|FlowControl|Delay MusicBoxDuration)
  (Audio|Components|Audio|AdjustVolume _laughingbaby 1.0 0.0 "Linear" :!class /Script/Engine.AudioComponent)
  (Utilities|FlowControl|Delay 1.0)
  (Audio|Components|Audio|Stop _laughingbaby)
  (Audio|Components|Audio|Play (Variables|Default|GetEnvironmentalAudio) 0.0))

(event Custom|BabyHappy
  (bind _environmentalaudio (Variables|Default|GetEnvironmentalAudio))
  ;[1 1 1] Baby stops crying and starts cooing
  (Audio|Components|Audio|SetSound _environmentalaudio "/Game/SpookyGame/Audio/Baby-room_lvl3_Audio/SFX_Baby/SFX_BabyCooing_loop_Cue.SFX_BabyCooing_loop_Cue")
  (Audio|Components|Audio|Play _environmentalaudio 0.0))

(event Custom|Cradle%20Baby%28PuzzleNotComplete%29
  (params (PlayerRef :type BP%20SG%20Player%20Object%20Reference))
  (bind _april_pawn (Variables|Default|GetApril%20Pawn))
  (bind _april_pawn_2 (Variables|Default|GetApril%20Pawn))
  (bind _sound_cradleinteract (Variables|Audio|GetSound_CradleInteract))
  (bind _sound_laughingbaby (Variables|Audio|GetSound_LaughingBaby))
  (bind _duration (Variables|/Script/Engine.SoundBase|GetDuration _sound_laughingbaby))
  (bind _returnvalue (/ _duration 2.0))
  ;[1 1 1] Cradle baby
  (Variables|/Game/SpookyGame/Blueprints/NPC/BP_April.BP_April_C|SetCanGiveHint (Variables|Default|GetApril%20Pawn) false)
  ;;[1 1 1] Stops enviromentalSound
  (Audio|Components|Audio|Stop (Variables|Default|GetEnvironmentalAudio))
  ;;[1 1 1] Plays cradle baby Sound
  (Audio|PlaySoundatLocation _sound_cradleinteract (Transformation|GetActorLocation) "0, 0, 0" 1.0 1.0 0.0 0 0 0 0)
  (Utilities|FlowControl|Delay (Variables|/Script/Engine.SoundBase|GetDuration _sound_cradleinteract))
  ;;[1 1 1] Plays Baby laughing Sound
  (Audio|PlaySoundatLocation _sound_laughingbaby (Transformation|GetActorLocation) "0, 0, 0" 1.0 1.0 0.0 0 0 0 0)
  (Utilities|FlowControl|Delay _returnvalue)
  ;;[1 1 1] Cabinet opens
  (Default|OpenCabinet (Variables|Default|GetBP_Cabinet))
  (Utilities|FlowControl|Delay _returnvalue)
  ;;[1 1 1] Baby Starts crying
  (Audio|Components|Audio|Play (Variables|Default|GetEnvironmentalAudio) 0.0)
  (Utilities|FlowControl|Delay 1.0)
  ;;[1 1 1] Cabinet closes
  (Default|CloseCabinet (Variables|Default|GetBP_Cabinet))
  ;[0.1038 1 0.7058] Scripted dialogue event
  (if (Variables|/Game/SpookyGame/Blueprints/NPC/BP_April.BP_April_C|GetPlayerHasInteractedWithBaby _april_pawn_2)
    (CallFunction|ExitScriptedDialogueEvent (Variables|Default|GetApril%20Pawn))
    (else
      (bind _sound_playing (CallFunction|BeginScriptedDialogueEvent _april_pawn_2 "/Game/SpookyGame/Audio/Baby-room_lvl3_Audio/SFX_Voice-Lines/SFX_Scripted-Dialogue/SFX_lvl3_DidYouNoticeTheCabinet_Cue.SFX_lvl3_DidYouNoticeTheCabinet_Cue"))
      (Utilities|FlowControl|Delay (Variables|/Script/Engine.SoundBase|GetDuration _sound_playing))
      (CallFunction|ExitScriptedDialogueEvent _april_pawn)
      (Variables|/Game/SpookyGame/Blueprints/NPC/BP_April.BP_April_C|SetPlayerHasInteractedWithBaby _april_pawn true)))
  (Variables|/Game/SpookyGame/Blueprints/Player/BP_SG_Player.BP_SG_Player_C|SetCanInteract PlayerRef true))

(event Custom|CradleBaby%28PuzzleCompleted%29
  (params (PlayerRef :type BP%20SG%20Player%20Object%20Reference))
  (bind _sound_cradleinteract (Variables|Audio|GetSound_CradleInteract))
  (bind _sound_laughingbaby (Variables|Audio|GetSound_LaughingBaby))
  ;[1 1 1] Cradle baby
  ;;[1 1 1] Stops enviromentalSound
  (Audio|Components|Audio|Stop (Variables|Default|GetEnvironmentalAudio))
  ;;[1 1 1] Plays cradle baby Sound
  (Audio|PlaySoundatLocation _sound_cradleinteract (Transformation|GetActorLocation) "0, 0, 0" 1.0 1.0 0.0 0 0 0 0)
  (Utilities|FlowControl|Delay (Variables|/Script/Engine.SoundBase|GetDuration _sound_cradleinteract))
  ;;[1 1 1] Plays Baby laughing Sound
  (Audio|PlaySoundatLocation _sound_laughingbaby (Transformation|GetActorLocation) "0, 0, 0" 1.0 1.0 0.0 0 0 0 0)
  (Utilities|FlowControl|Delay (Variables|/Script/Engine.SoundBase|GetDuration _sound_laughingbaby))
  ;;[1 1 1] Start enviromentalSound
  (Audio|Components|Audio|Play (Variables|Default|GetEnvironmentalAudio) 0.0)
  (Pawn|Components|CharacterMovement|SetMovementMode (Variables|/Script/Engine.Character|GetCharacterMovement PlayerRef) "MOVE_Walking" 0)
  (Variables|/Game/SpookyGame/Blueprints/Player/BP_SG_Player.BP_SG_Player_C|SetCanInteract PlayerRef true))

(event Custom|Baby%20gets%20Teddy
  ;[1 1 1] Baby gets Teddy
  (Audio|PlaySoundatLocation 0 (Transformation|GetActorLocation) "0, 0, 0" 1.0 1.0 0.0 0 0 0 0)
  (Audio|Components|Audio|Stop (Variables|Default|GetEnvironmentalAudio))
  (Development|PrintString "Baby reached Nirvana"))

(event EventBeginPlay
  (|CallParentFunction)
  (bind _returnvalue (Actor|GetActorOfClass "/Game/SpookyGame/Blueprints/Objects/BP_InteractableObject_Cabinet.BP_InteractableObject_Cabinet_C"))
  (Variables|Default|SetBP_Cabinet _returnvalue)
  (bind _returnvalue_2 (Actor|GetActorOfClass "/Game/SpookyGame/Blueprints/NPC/BP_April.BP_April_C"))
  (Variables|Default|SetApril%20Pawn _returnvalue_2))

(event EventTriggerEvent
  (params (PlayerREF :type BP%20SG%20Player%20Object%20Reference))
  (bind _charactermovement (Variables|/Script/Engine.Character|GetCharacterMovement PlayerREF))
  (Variables|/Game/SpookyGame/Blueprints/Player/BP_SG_Player.BP_SG_Player_C|SetCanInteract PlayerREF false)
  (if (Variables|/Game/SpookyGame/Blueprints/Player/BP_SG_Player.BP_SG_Player_C|GetbHasTeddy? PlayerREF)
    (CallFunction|BabyGetsTeddy)
    (bind _doortonextlevel (Variables|Default|GetDoorToNextLevel)
      (:then
        (Default|OpenDoor _doortonextlevel)
        (Variables|/Game/SpookyGame/Blueprints/Player/BP_SG_Player.BP_SG_Player_C|SetCanInteract PlayerREF true))
      (:else))
    (elif (Variables|/Game/SpookyGame/Blueprints/Objects/BP_PuzzlePawn.BP_PuzzlePawn_C|GetIsPuzzleCompleted (Variables|Default|GetPianoPuzzle))
      (Pawn|Components|CharacterMovement|DisableMovement _charactermovement)
      (CallFunction|CradleBaby(PuzzleCompleted) PlayerREF)
      (else
        (Pawn|Components|CharacterMovement|DisableMovement _charactermovement)
        (CallFunction|CradleBaby(PuzzleNotComplete) PlayerREF)))))

(fn ConstructionScript
  (|CallParentFunction))