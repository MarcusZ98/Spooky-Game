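; BP_Triggering is an actor for a radio puzzle that plays a clue sound when the left and right channel values both equal one.
; Custom events step each channel up or down and restart the fail sound in place of the radio sound that starts on BeginPlay.
; Tick checks the combination, then plays the clue, resets the right channel and destroys the radio and fail components.
; Separate events switch between left and right point sounds.
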(event Custom|Play%20Left
  (Audio|Components|Audio|Stop (Variables|Default|GetPointSoundRight))
  (Audio|Components|Audio|Play (Variables|Default|GetPointSoundLeft) 0.0)
  (Development|PrintString "left"))

(event Custom|DecreaseLeft
  (bind _output_get (Variables|Default|Setradiochannel_left (+ -1 (Variables|Default|Getradiochannel_left))))
  (Development|PrintString (Utilities|String|ToString(Integer) _output_get))
  (Audio|Components|Audio|Stop (Variables|Default|GetPointSoundRadioFail))
  (Audio|Components|Audio|Play (Variables|Default|GetPointSoundRadioFail) 0.0))

(event Custom|IncreaseRight
  (bind _output_get (Variables|Default|Setradiochannel_right (+ 1 (Variables|Default|Getradiochannel_right))))
  (Development|PrintString (Utilities|String|ToString(Integer) _output_get))
  (Audio|Components|Audio|Stop (Variables|Default|GetPointSoundRadioFail))
  (Audio|Components|Audio|Play (Variables|Default|GetPointSoundRadioFail) 0.0))

(event Custom|IncreaseLeft
  (bind _output_get (Variables|Default|Setradiochannel_left (+ 1 (Variables|Default|Getradiochannel_left))))
  (Development|PrintString (Utilities|String|ToString(Integer) _output_get))
  (Audio|Components|Audio|Stop (Variables|Default|GetPointSoundRadioFail))
  (Audio|Components|Audio|Play (Variables|Default|GetPointSoundRadioFail) 0.0))

(event Custom|Play%20Right
  (Audio|Components|Audio|Stop (Variables|Default|GetPointSoundLeft))
  (Audio|Components|Audio|Play (Variables|Default|GetPointSoundRight) 0.0)
  (Development|PrintString "right"))

(event Custom|DecreaseRight
  (bind _output_get (Variables|Default|Setradiochannel_right (+ -1 (Variables|Default|Getradiochannel_right))))
  (Development|PrintString (Utilities|String|ToString(Integer) _output_get))
  (Audio|Components|Audio|Stop (Variables|Default|GetPointSoundRadioFail))
  (Audio|Components|Audio|Play (Variables|Default|GetPointSoundRadioFail) 0.0))

(event EventBeginPlay
  (Audio|Components|Audio|Play (Variables|Default|GetPointSoundRadio) 0.0)
  (Audio|Components|Audio|Stop (Variables|Default|GetPointSoundRadioClue)))

(event Collision|EventActorBeginOverlap
  (params (OtherActor :type Actor%20Object%20Reference)))

(event EventTick
  (params (DeltaSeconds :type Float%20%28single-precision%29))
  (if (and (== (Variables|Default|Getradiochannel_right) 1) (== (Variables|Default|Getradiochannel_left) 1))
    (Audio|Components|Audio|Stop (Variables|Default|GetPointSoundRadio))
    (Audio|Components|Audio|Play (Variables|Default|GetPointSoundRadioClue) 0.0)
    (Development|PrintString "You get clue")
    (Variables|Default|Setradiochannel_right 0)
    (Components|DestroyComponent (Variables|Default|GetPointSoundRadioFail))))

(fn ConstructionScript)