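; BP_PuzzlePawn_Piano is a puzzle pawn for a piano where W, A, S and D each play a note.
; Each press is checked against KeyCodeSheet by the current sequence length, and a wrong key clears progress.
; Four correct keys complete the puzzle, switching ambient audio, calming the baby, stopping the music box, destroying its mesh and the door, and opening the cabinet.
; Completion, or triggering once completed, repossesses the player.
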(event EventTriggerEvent
  (params (PlayerREF :type BP%20SG%20Player%20Object%20Reference))
  (|CallParentFunction PlayerREF)
  (if (Variables|Default|GetIsPuzzleCompleted)
    (CallFunction|RepossessPlayer)))

(event Input|KeyboardEvents|A
  (params (Key :type Key%20Structure :default "None"))
  (:Pressed
    (Audio|Components|Audio|Play (Variables|Default|GetA) 0.0)
    (CallFunction|ValidateNoteSequence Key)))

(event Input|KeyboardEvents|S
  (params (Key :type Key%20Structure :default "None"))
  (:Pressed
    (Audio|Components|Audio|Play (Variables|Default|GetC) 0.0)
    (CallFunction|ValidateNoteSequence Key)))

(event Input|KeyboardEvents|D
  (params (Key :type Key%20Structure :default "None"))
  (:Pressed
    (Audio|Components|Audio|Play (Variables|Default|GetE) 0.0)
    (CallFunction|ValidateNoteSequence Key)))

(event Input|KeyboardEvents|W
  (params (Key :type Key%20Structure :default "None"))
  (:Pressed
    (Audio|Components|Audio|Play (Variables|Default|GetD) 0.0)
    (CallFunction|ValidateNoteSequence Key)))

(fn ConstructionScript
  (|CallParentFunction))

(fn ValidateNoteSequence
  (params (Key :type Key%20Structure :default "None"))
  (bind _currentnotesequence (Variables|Default|GetCurrentNoteSequence))
  (if (== (Utilities|Array|Get(acopy) (Variables|Default|GetKeyCodeSheet) (Utilities|Array|Length (Variables|Default|GetCurrentNoteSequence))) Key)
    ;[1 1 1] If keynote is right it adds the key to "CurrentNoteSequence"
    (Utilities|Array|Add _currentnotesequence Key)
    (Development|PrintString "Correct key")
    (if (== (Utilities|Array|Length _currentnotesequence) 4)
      (CallFunction|PuzzleComplete))
    (else
      ;[1 1 1] If the keynote is not right clears the "CurrentNoteSequence"
      (Utilities|Array|Clear (Variables|Default|GetCurrentNoteSequence))
      (Development|PrintString "Wrong key"))))

(fn PuzzleComplete
  (bind _environmentalaudio (Variables|Default|GetEnvironmentalAudio))
  (|CallParentFunction)
  (Development|PrintString "Piano Puzzle done")
  ;[1 1 1] Sets new enviromental sound to the completedpuzzle enviromentalSound
  (Audio|Components|Audio|SetSound _environmentalaudio "/Game/SpookyGame/Audio/Baby-room_lvl3_Audio/SFX_Piano/SFX_piano-loop_FULL_Cue.SFX_piano-loop_FULL_Cue")
  (Audio|Components|Audio|Play _environmentalaudio 0.0)
  ;[1 1 1] Baby Stops crying
  (Default|BabyHappy (Variables|Default|GetBaby))
  ;[1 1 1] MusicBox Stops playing
  (Default|StopPlaying (Variables|Default|GetMusicBox))
  (Variables|Default|SetIsPuzzleCompleted true)
  (CallFunction|RepossessPlayer)
  (Components|DestroyComponent (Variables|Default|GetStaticMesh))
  (Actor|DestroyActor (Variables|Default|GetDoor))
  ;[1 1 1] Opens Cabinet
  (Default|OpenCabinet (Variables|Default|GetCabinet)))