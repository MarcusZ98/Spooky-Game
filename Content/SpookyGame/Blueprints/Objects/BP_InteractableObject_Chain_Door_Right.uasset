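; Right-hand chain door interactable that slides open when the player enters a directional key code, and also triggers the left door.
; Triggering runs the parent interaction and stores the player, unless the door has already moved.
; Arrow key events advance a step counter through Up, Up, Left, Down, Right, resetting on mistakes.
; Completion moves the mesh sideways, repossesses the player, and triggers the left door found by class, flagging it moved.
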(event EventBeginPlay
  (|CallParentFunction) ; This node is disabled and will not be called.\nDrag off pins to build functionality.
)

(event Collision|EventActorBeginOverlap
  (params (OtherActor :type Actor%20Object%20Reference))
  (|CallParentFunction OtherActor) ; This node is disabled and will not be called.\nDrag off pins to build functionality.
)

(event EventTick
  (params (DeltaSeconds :type Float%20%28single-precision%29))
  (|CallParentFunction DeltaSeconds) ; This node is disabled and will not be called.\nDrag off pins to build functionality.
)

(event EventTriggerEvent
  (params (PlayerREF :type BP%20SG%20Player%20Object%20Reference))
  (if (not (Variables|Default|GetRight_Moved?))
    (|CallParentFunction PlayerREF)
    (Variables|Default|SetPlayer%20REF PlayerREF)))

(event Input|KeyboardEvents|Left
  (params (Key :type Key%20Structure :default "None"))
  (:Pressed
    (if (== (Variables|Default|GetCorrect_Inputs) 2)
      (Variables|Default|SetCorrect_Inputs 3)
      (else
        (Variables|Default|SetCorrect_Inputs 0)))))

(event Input|KeyboardEvents|Right
  (params (Key :type Key%20Structure :default "None"))
  (:Pressed
    (if (== (Variables|Default|GetCorrect_Inputs) 4)
      (Variables|Default|SetCorrect_Inputs 5)
      (Utilities|FlowControl|Sequence
        (:then_0
          (Utilities|FlowControl|DoOnce false
            (:Completed
              (Components|MoveComponentTo (Variables|Default|GetStaticMesh) "0.000000,400.000000,0.000000" "0, 0, 0" false false 2.0 false)
              (Variables|Default|SetRight_Moved? true)
              (CallFunction|RepossessPlayer))))
        (:then_1
          (Utilities|FlowControl|DoOnce false
            (:Completed
              (bind _returnvalue (Actor|GetActorOfClass "/Game/SpookyGame/Blueprints/Objects/BP_InteractableObject_Chain_Door_Left.BP_InteractableObject_Chain_Door_Left_C"))
              (Default|TriggerEvent _returnvalue)
              (Variables|/Game/SpookyGame/Blueprints/Objects/BP_InteractableObject_Chain_Door_Left.BP_InteractableObject_Chain_Door_Left_C|SetLeft_Moved? _returnvalue true)))))
      (else
        (Variables|Default|SetCorrect_Inputs 0)))))

(event Input|KeyboardEvents|Up
  (params (Key :type Key%20Structure :default "None"))
  (:Pressed
    (if (== (Variables|Default|GetCorrect_Inputs) 0)
      (Variables|Default|SetCorrect_Inputs 1)
      (elif (== (Variables|Default|GetCorrect_Inputs) 1)
        (Variables|Default|SetCorrect_Inputs 2)
        (else
          (Variables|Default|SetCorrect_Inputs 0))))))

(event Input|KeyboardEvents|Down
  (params (Key :type Key%20Structure :default "None"))
  (:Pressed
    (if (== (Variables|Default|GetCorrect_Inputs) 3)
      (Variables|Default|SetCorrect_Inputs 4)
      (else
        (Variables|Default|SetCorrect_Inputs 0)))))

(fn ConstructionScript
  (|CallParentFunction))