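; Interactable cabinet that gives the player a teddy, with a 2D sound, the first time it is triggered while open.
; Triggering it while closed prints a debug message and plays interaction audio, locked by a DoOnce until the clip finishes.
; OpenCabinet and CloseCabinet set the open state and play positional sounds.
; Opening also wraps its delayed sound in a focus event, which exits after the sound ends.
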(event Custom|Open%20Cabinet
  (Variables|Default|SetbIsOpen? true)
  (CallFunction|BeginFocusEvent (Variables|Audio|GetSound_OpenCabinet) true 0.1 2.5)
  (Utilities|FlowControl|Delay 2.5)
  (Audio|PlaySoundatLocation (Variables|Audio|GetSound_OpenCabinet) (Transformation|GetWorldLocation (Variables|Default|GetDefaultSceneRoot)) "0, 0, 0" 1.0 1.0 0.0 0 0 0 0)
  (Utilities|FlowControl|Delay (+ (Variables|/Script/Engine.SoundBase|GetDuration (Variables|Audio|GetSound_OpenCabinet)) 0.3))
  (CallFunction|ExitFocusEvent 2.0))

(event Custom|Close%20Cabinet
  (Variables|Default|SetbIsOpen? false)
  (Audio|PlaySoundatLocation (Variables|Audio|GetSound_CloseCabinet) (Transformation|GetWorldLocation (Variables|Default|GetDefaultSceneRoot)) "0, 0, 0" 1.0 1.0 0.0 0 0 0 0))

(event EventBeginPlay)

(event Collision|EventActorBeginOverlap
  (params (OtherActor :type Actor%20Object%20Reference))
  (|CallParentFunction OtherActor) ; This node is disabled and will not be called.\nDrag off pins to build functionality.
)

(event EventTick
  (params (DeltaSeconds :type Float%20%28single-precision%29))
  (|CallParentFunction DeltaSeconds) ; This node is disabled and will not be called.\nDrag off pins to build functionality.
)

(event EventTriggerEvent
  (params (PlayerREF :type BP%20SG%20Player%20Object%20Reference))
  (bind _interactaudio (Variables|Default|GetInteractAudio))
  (if (Variables|Default|GetbIsOpen?)
    (Utilities|FlowControl|DoOnce false
      (:Completed
        (Default|ReciveTeddy PlayerREF)
        (Audio|PlaySound2D 0 1.0 1.0 0.0 0 0)))
    (else
      (Utilities|FlowControl|DoOnce false :!label _label
        (:Completed
          (Development|PrintString "Cabinet closed")
          (Audio|Components|Audio|Play _interactaudio 0.0)
          (Utilities|FlowControl|Delay (Variables|/Script/Engine.SoundBase|GetDuration (Variables|/Script/Engine.AudioComponent|GetSound _interactaudio)))
          (goto _label Reset))))))

(fn ConstructionScript
  (|CallParentFunction))