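; BP_InteractableObject is an interactable world object that delivers audio hints and descriptions.
; TriggerEvent passes its InteractSound to the GiveNarrativeHint function on BPApril, reached through the GameState.
; A separate TriggerAudioDescription function plays a supplied description sound at the location of the EnvironmentalAudio component.
; BeginPlay, overlap and Tick are unused stubs, so both behaviors depend on being called.
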(event EventBeginPlay
  (|CallParentFunction) ; This node is disabled and will not be called.\nDrag off pins to build functionality.
)

(event Collision|EventActorBeginOverlap
  (params (OtherActor :type Actor%20Object%20Reference))
  (|CallParentFunction OtherActor) ; This node is disabled and will not be called.\nDrag off pins to build functionality.
)

(event EventTick
  (params (DeltaSeconds :type Float%20%28single-precision%29))
  (|CallParentFunction DeltaSeconds) ; This node is disabled and will not be called.\nDrag off pins to build functionality.
)

(event EventTriggerEvent
  (params (PlayerREF :type BP%20SG%20Player%20Object%20Reference))
  (Default|GiveNarrativeHint (Variables|/Game/SpookyGame/Blueprints/FrameWork/BP_SG_GameState.BP_SG_GameState_C|GetBP_April (Variables|Default|GetGameState)) (Variables|Default|GetInteractSound)))

(fn ConstructionScript
  (|CallParentFunction))

(fn TriggerAudioDescription
  (params (ObjectDescriptionSound :type Sound%20Cue%20Object%20Reference))
  (Audio|PlaySoundatLocation ObjectDescriptionSound (Transformation|GetWorldLocation (Variables|Default|GetEnvironmentalAudio)) "0, 0, 0" 1.0 1.0 0.0 0 0 0 0))