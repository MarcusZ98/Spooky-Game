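; BP_InteractableObject_TutorialTools is the tutorial tool pickup that grants the player their tools, including the geiger, when triggered.
; On TriggerEvent it waits a tick, sets PlayerHasTools, picks dialogue on the BP_DialogueManager cached at BeginPlay, starts it and destroys itself.
; If the tutorial closet actor still exists it sets a specific dialogue asset; otherwise it queues its own Dialogues list.
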(event EventBeginPlay
  (|CallParentFunction)
  (bind _returnvalue (Actor|GetActorOfClass "/Game/SpookyGame/Blueprints/Dialogue/BP_DialogueManager.BP_DialogueManager_C"))
  (Variables|Default|SetDM _returnvalue))

(event Collision|EventActorBeginOverlap
  (params (OtherActor :type Actor%20Object%20Reference)))

(event EventTick
  (params (DeltaSeconds :type Float%20%28single-precision%29)))

(event EventTriggerEvent
  (params (PlayerREF :type BP%20SG%20Player%20Object%20Reference))
  (Utilities|FlowControl|DelayUntilNextTick)
  (Utilities|FlowControl|Sequence
    (:then_0
      (Development|PrintString "You now have geiger"))
    (:then_1
      (Variables|Default|SetplayerHasTools true))
    (:then_2
      (bind _returnvalue (Actor|GetActorOfClass "/Game/SpookyGame/Blueprints/Objects/BP_InteractableObject_TutorialCloset.BP_InteractableObject_TutorialCloset_C"))
      (if (Utilities|IsValid _returnvalue)
        (Default|SetDialogue (Variables|Default|GetDM) "/Game/SpookyGame/Blueprints/Dialogue/Tutorial/Dialogues/DA_Dialogue_3.DA_Dialogue_3")
        (else
          (Default|QueueDialogues (Variables|Default|GetDM) (Variables|Default|GetDialogues)))))
    (:then_3
      (Default|StartDialogue (Variables|Default|GetDM)))
    (:then_4
      (Actor|DestroyActor))))

(fn ConstructionScript
  (|CallParentFunction))