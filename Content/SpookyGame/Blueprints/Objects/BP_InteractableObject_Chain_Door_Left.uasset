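; Left chain door interactable that opens when the player enters a fixed directional-key sequence.
; Triggering hands off to the parent class and stores the player until the door has moved.
; A counter advances on each correct key and resets on a wrong one; completion slides two meshes apart, repossesses the player and switches to door and room-shake audio.
; Logic to trigger the right-hand door is present but never runs.
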(event EventBeginPlay
  (|CallParentFunction) ; This node is disabled and will not be called.\nDrag off pins to build functionality.
)

(event Collision|EventActorBeginOverlap
  (params (OtherActor :type Actor%20Object%20Reference))
  (|CallParentFunction OtherActor) ; This node is disabled and will not be called.\nDrag off pins to build functionality.
)

(event EventTick
  (params (DeltaSeconds :type Float%20%28single-precision%29))
  (|CallParentFunction DeltaSeconds) ; This node is disabled and will not be called.\nDrag off pins to build functionality.
)

(event EventTriggerEvent
  (params (PlayerREF :type BP%20SG%20Player%20Object%20Reference))
  (if (not (Variables|Default|GetLeft_Moved?))
    (|CallParentFunction PlayerREF)
    (Variables|Default|SetPlayer%20REF PlayerREF)))

(event Input|KeyboardEvents|Left
  (params (Key :type Key%20Structure :default "None"))
  (:Pressed
    (if (== (Variables|Default|GetCorrect_Inputs) 2)
      (Variables|Default|SetCorrect_Inputs 3)
      (else
        (Variables|Default|SetCorrect_Inputs 0)))))

(event Input|KeyboardEvents|Right
  (params (Key :type Key%20Structure :default "None"))
  (bind _environmentalaudio (Variables|Default|GetEnvironmentalAudio))
  (:Pressed
    (if (== (Variables|Default|GetCorrect_Inputs) 4)
      (Variables|Default|SetCorrect_Inputs 5)
      (Utilities|FlowControl|Sequence
        (:then_0
          (Utilities|FlowControl|DoOnce false
            (:Completed
              (Utilities|FlowControl|Sequence
                (:then_0
                  (Components|MoveComponentTo (Variables|Default|GetStaticMesh) "0.000000,-800.000000,0.000000" "0.000000,90.000000,0.000000" false false 3.0 false))
                (:then_1
                  (Components|MoveComponentTo (Variables|Default|GetStaticMesh2) "0.000000,800.000000,0.000000" "0.000000,90.000000,0.000000" false false 3.0 false)
                  (Variables|Default|SetLeft_Moved? true))
                (:then_2
                  (CallFunction|RepossessPlayer))
                (:then_3
                  (Audio|Components|Audio|Stop (Variables|Default|GetEnvironmentalAudio))
                  (Audio|Components|Audio|Play (Variables|Default|GetDoorIdleAudio) 0.0)
                  (Utilities|FlowControl|DoOnce false
                    (:Completed
                      (Audio|Components|Audio|SetSound _environmentalaudio "/Game/SpookyGame/Audio/Captain/SFX/SFX_Room_Shake.SFX_Room_Shake")
                      (Audio|Components|Audio|Play _environmentalaudio 0.0)))))))))
      (else
        (Variables|Default|SetCorrect_Inputs 0)))))

(event Input|KeyboardEvents|Up
  (params (Key :type Key%20Structure :default "None"))
  (:Pressed
    (if (== (Variables|Default|GetCorrect_Inputs) 0)
      (Variables|Default|SetCorrect_Inputs 1)
      (elif (== (Variables|Default|GetCorrect_Inputs) 1)
        (Variables|Default|SetCorrect_Inputs 2)
        (else
          (Variables|Default|SetCorrect_Inputs 0))))))

(event Input|KeyboardEvents|Down
  (params (Key :type Key%20Structure :default "None"))
  (:Pressed
    (if (== (Variables|Default|GetCorrect_Inputs) 3)
      (Variables|Default|SetCorrect_Inputs 4)
      (else
        (Variables|Default|SetCorrect_Inputs 0)))))

(fn ConstructionScript
  (|CallParentFunction))