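; Interactable door that plays a locked sound until opened, then loads a configured level when triggered.
; OpenDoor sets the open flag, plays a sound and uses a timeline to lerp the mesh from its current rotation toward 180 degrees of yaw past its BeginPlay rotation.
; TriggerEvent checks that flag to either open LevelToOpen by name with the door sound or play the locked sound.
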(event Custom|Open%20Door
  (bind _initialdoorrotation (Variables|Default|GetInitialDoorRotation))
  (Variables|Default|SetbIsOpen? true)
  (Audio|PlaySoundatLocation (Variables|Audio|GetSound_OpenDoor) (Transformation|GetActorLocation) "0, 0, 0" 1.0 1.0 0.0 0 0 0 0)
  (bind _alpha (Timeline|Timeline Play)
    (:Update
      (Transformation|SetRelativeRotation (Variables|Default|GetStaticMesh) (Math|Rotator|Lerp(Rotator) (Variables|/Script/Engine.SceneComponent|GetRelativeRotation (Variables|Default|GetStaticMesh)) (Math|Rotator|MakeRotator (.roll _initialdoorrotation) (.pitch _initialdoorrotation) (+ (.yaw _initialdoorrotation) 1.8e+02)) _alpha true) false false))))

(event EventTriggerEvent
  (params (PlayerREF :type BP%20SG%20Player%20Object%20Reference))
  (if (Variables|Default|GetbIsOpen?)
    (Audio|PlaySoundatLocation (Variables|Audio|GetSound_OpenDoor) (Transformation|GetActorLocation) "0, 0, 0" 1.0 1.0 0.0 0 0 0 0)
    (Game|OpenLevel(byName) (Variables|Default|GetLevelToOpen))
    (else
      (Audio|PlaySoundatLocation (Variables|Audio|GetSound_DoorLocked) (Transformation|GetActorLocation) "0, 0, 0" 1.0 1.0 0.0 0 0 0 0))))

(event EventBeginPlay
  (|CallParentFunction)
  (Variables|Default|SetInitialDoorRotation (Variables|/Script/Engine.SceneComponent|GetRelativeRotation (Variables|Default|GetStaticMesh))))

(fn ConstructionScript
  (|CallParentFunction))