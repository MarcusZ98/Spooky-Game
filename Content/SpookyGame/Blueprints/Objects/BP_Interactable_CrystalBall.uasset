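; Crystal ball interactable that drives the level 5 ending through the level's event manager.
; Player overlap with its dialogue collider logs "Player destroyed artifact" via the game instance, fires CrystalOrbEnding after a short delay, then removes the collider.
; A timeline adjusts environmental and looping cellar audio volume, and its update branch briefly disables player input.
; Space bar calls KillApril on the manager and quits the game after a delay.
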(event OnComponentBeginOverlap(DialogueCol)
  (params (OverlappedComponent :type Primitive%20Component%20Object%20Reference) (OtherActor :type Actor%20Object%20Reference) (OtherComp :type Primitive%20Component%20Object%20Reference) (OtherBodyIndex :type Integer) (bFromSweep :type Boolean) (SweepResult :type Hit%20Result%20Structure%20%28by%20ref%29))
  (bind _returnvalue (Game|GetPlayerController 0))
  (if (== OtherActor (Game|GetPlayerCharacter 0))
    (Utilities|FlowControl|Sequence
      (:then_0
        (Utilities|FlowControl|Delay 2.0)
        (bind _returnvalue_2 (Actor|GetActorOfClass "/Game/SpookyGame/Blueprints/NPC/BP_lvl5_EventManager.BP_lvl5_EventManager_C"))
        (Default|CrystalOrbEnding _returnvalue_2)
        (Components|DestroyComponent (Variables|Default|GetDialogueCol)))
      (:then_1
        (bind _assg_game_instance (Utilities|Casting|CastToSG_GameInstance (Game|GetGameInstance)))
        (Class|SGGameInstance|WritetoFile _assg_game_instance "Player destroyed artifact")
        (bind _volume_over_time (Timeline|Timeline Play)
          (:Update
            (Utilities|FlowControl|Sequence
              (:then_0
                (Audio|Components|Audio|SetVolumeMultiplier (Variables|Default|GetEnvironmentalAudio) _volume_over_time :!class /Script/Engine.AudioComponent))
              (:then_1
                (Audio|Components|Audio|SetVolumeMultiplier (Variables|Default|GetSFX_Cellar_Ambient_Loop) _volume_over_time :!class /Script/Engine.AudioComponent))
              (:then_2
                (Input|DisableInput _returnvalue)
                (Utilities|FlowControl|Delay 4.0)
                (Input|EnableInput _returnvalue)))))))))

(event EventBeginPlay
  (|CallParentFunction)
  (Audio|Components|Audio|Play (Variables|Default|GetSFX_Cellar_Ambient_Loop) 0.0))

(event EventTriggerEvent
  (params (PlayerREF :type BP%20SG%20Player%20Object%20Reference))
  (|CallParentFunction PlayerREF))

(event Input|KeyboardEvents|SpaceBar
  (params (Key :type Key%20Structure :default "None"))
  (:Pressed
    (bind _returnvalue (Actor|GetActorOfClass "/Game/SpookyGame/Blueprints/NPC/BP_lvl5_EventManager.BP_lvl5_EventManager_C"))
    (Default|KillApril _returnvalue)
    (Utilities|FlowControl|Delay 8.5)
    (Game|QuitGame 0 "Quit" false)))

(fn ConstructionScript
  (|CallParentFunction))