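; Possessable audio-driven combat tutorial where the player counters enemy attacks heard from the right, center or left, then regains the normal player pawn.
; Each round plays a random directional attack sound, which must be answered with the matching D/W/A or arrow key before it ends.
; Wrong or late counters play failure cues and start another round.
; Reaching the required hit count plays a clear cue, exits audio focus, repossesses the player and destroys the actor.
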(event Custom|ExitCombat
  ;[1 1 1] Exit Combat
  (bind _asbp_sg_game_mode (Utilities|Casting|CastToBP_SG_GameMode (Game|GetGameMode)))
  (Pawn|Possess (Game|GetPlayerController 0) (Variables|/Game/SpookyGame/Blueprints/FrameWork/BP_SG_GameMode.BP_SG_GameMode_C|GetPlayer _asbp_sg_game_mode)))

(event Custom|Play%20Enemy%20Attack%20Sound
  (params (Index :type Integer))
  (bind _audioattackarray (Variables|Audio|GetAudioAttackArray))
  (bind _output (Utilities|Array|Get(acopy) _audioattackarray Index))
  (Audio|Components|Audio|Play _output 0.0)
  (Utilities|FlowControl|Delay (Variables|/Script/Engine.SoundBase|GetDuration (Variables|/Script/Engine.AudioComponent|GetSound _output)))
  (if (Variables|Default|GetbCanCounterAttack)
    (Variables|Default|SetbLateAttack? true)
    (CallFunction|HitPlayer)))

(event EventBeginPlay
  (CallFunction|BeginFocusEvent "/Game/SpookyGame/Blueprints/Dialogue/Tutorial/SoundFiles/Combat/Cue_TutorialCombat_Attack.Cue_TutorialCombat_Attack" true 0.0 2.0 (Utilities|Struct|MakeSTR_MapWrapper (Utilities|Map|MakeMap "/Game/SpookyGame/Blueprints/FrameWork/SC_Enemy.SC_Enemy" 1.0)))
  (Audio|PlaySoundatLocation "/Game/SpookyGame/Audio/Enemy/combat_begin.combat_begin" (Transformation|GetActorLocation) "0, 0, 0" 1.0 1.0 0.0 0 0 0 0)
  ;[1 1 1] Intro combat
  (Utilities|FlowControl|Delay 4.0)
  (Variables|Audio|SetAudioAttackArray (Utilities|Array|MakeArray (Variables|Default|GetRightAudio) (Variables|Default|GetCenterAudio) (Variables|Default|GetLeftAudio)))
  (Variables|Audio|SetAudioCounterArray (Utilities|Array|MakeArray (Variables|Default|GetRightAudioPC) (Variables|Default|GetCenterAudioPC) (Variables|Default|GetLeftAudioPC)))
  (bind _index (CallFunction|GetRandomIndex))
  (CallFunction|PlayEnemyAttackSound _index)
  (Variables|Default|SetbCanCounterAttack true))

(event Input|KeyboardEvents|Escape
  (params (Key :type Key%20Structure :default "None"))
  (bind _bp_mainmenucomponent (Variables|Default|GetBP_MainMenuComponent))
  (:Pressed
    (Utilities|FlowControl|FlipFlop
      (:A
        (Default|OpenMenu _bp_mainmenucomponent))
      (:B
        (Default|CloseMenu _bp_mainmenucomponent)))))

(event Input|KeyboardEvents|W
  (params (Key :type Key%20Structure :default "None"))
  ;[1 1 1] Counter
  (:Pressed
    (CallFunction|CounterAttack 1)))

(event Input|KeyboardEvents|D
  (params (Key :type Key%20Structure :default "None"))
  ;[1 1 1] Counter
  (:Pressed
    (CallFunction|CounterAttack)))

(event Input|KeyboardEvents|Right
  (params (Key :type Key%20Structure :default "None"))
  ;[1 1 1] Counter
  (:Pressed
    (CallFunction|CounterAttack)))

(event Input|KeyboardEvents|A
  (params (Key :type Key%20Structure :default "None"))
  ;[1 1 1] Counter
  (:Pressed
    (CallFunction|CounterAttack 2)))

(event Input|KeyboardEvents|Left
  (params (Key :type Key%20Structure :default "None"))
  ;[1 1 1] Counter
  (:Pressed
    (CallFunction|CounterAttack 2)))

(event Input|KeyboardEvents|Up
  (params (Key :type Key%20Structure :default "None"))
  ;[1 1 1] Counter
  (:Pressed
    (CallFunction|CounterAttack 1)))

(fn ConstructionScript)

(fn GetRandomIndex
  (bind _output_get (Variables|Default|SetCurrentIndex (.OutIndex (Utilities|Array|Random (Variables|Audio|GetAudioAttackArray)))))
  (return _output_get))

(fn CounterAttack
  (params (Index :type Integer))
  (LocalVariables|SetCounterIndex Index)
  (if (Variables|Default|GetbCanCounterAttack)
    (Audio|Components|Audio|Play (Utilities|Array|Get(acopy) (Variables|Audio|GetAudioCounterArray) Index) 0.0)
    (Variables|Default|SetbCanCounterAttack false)
    (if (== (LocalVariables|GetCounterIndex) (Variables|Default|GetCurrentIndex))
      (Utilities|Time|SetTimerbyFunctionName 0 "HitEnemy" 0.3)
      (else
        (CallFunction|MissEnemy)))))

(fn StartCombat
  (bind _index (CallFunction|GetRandomIndex))
  (CallFunction|PlayEnemyAttackSound _index)
  (Variables|Default|SetbCanCounterAttack true))

(fn HitEnemy
  (bind _audioattackarray (Variables|Audio|GetAudioAttackArray))
  (bind _currentindex (Variables|Default|GetCurrentIndex))
  (bind _output (Utilities|Array|Get(acopy) _audioattackarray _currentindex))
  (Math|Integer|IncrementInt (Variables|Default|GetCurrentEnemiesDefeated)
    (:%20%20
      (Audio|Components|Audio|Stop _output)
      (Development|PrintString "EnemyHit")
      (if (== (Variables|Default|GetCurrentEnemiesDefeated) (Variables|Default|GetEnemiesToDefeat))
        (Utilities|Time|SetTimerbyFunctionName 0 "EndCombat" 2.0)
        (else
          (Audio|PlaySoundatLocation (LocalVariables|GetAttackHitSuccess) (Transformation|GetWorldLocation _output) "0, 0, 0" 1.0 1.0 0.0 0 0 0 0)
          (Utilities|Time|SetTimerbyFunctionName 0 "StartCombat" (+ (Variables|/Script/Engine.SoundBase|GetDuration (LocalVariables|GetAttackHitSuccess)) 2.0)))))))

(fn MissEnemy
  (Variables|Default|SetbHasMissed? true)
  (CallFunction|HitPlayer))

(fn EndCombat
  (bind _returnvalue (Audio|SpawnSound2D "/Game/SpookyGame/Blueprints/Dialogue/Tutorial/SoundFiles/Combat/Cue_TutorialCombat_Clear.Cue_TutorialCombat_Clear" 1.0 1.0 0.0 0))
  (Utilities|Time|SetTimerbyFunctionName 0 "ReturnToPlayer" (Variables|/Script/Engine.SoundBase|GetDuration (Variables|/Script/Engine.AudioComponent|GetSound _returnvalue)))
  (CallFunction|ExitFocusEvent 2.0))

(fn ReturntoPlayer
  (bind _asbp_sg_game_mode (Utilities|Casting|CastToBP_SG_GameMode (Game|GetGameMode)))
  (Pawn|Possess (Game|GetPlayerController 0) (Variables|/Game/SpookyGame/Blueprints/FrameWork/BP_SG_GameMode.BP_SG_GameMode_C|GetPlayer _asbp_sg_game_mode))
  (Actor|DestroyActor))

(fn HitPlayer
  (Variables|Default|SetbCanCounterAttack false)
  (bind _result (Math|Integer|DecrementInt (Variables|Default|GetHealth))
    (:%20%20
      (Math|Integer|IncrementInt _result
        (:%20%20
          (Development|PrintString "Player Hit")
          (if (Variables|Default|GetbHasMissed?)
            (bind _returnvalue (Audio|SpawnSound2D "/Game/SpookyGame/Blueprints/Dialogue/Tutorial/SoundFiles/Combat/Cue_TutorialCombat_FailedAttack.Cue_TutorialCombat_FailedAttack" 1.0 1.0 0.0 0))
            (LocalVariables|SetAudioComponent _returnvalue)
            (else
              (bind _returnvalue_2 (Audio|SpawnSound2D "/Game/SpookyGame/Blueprints/Dialogue/Tutorial/SoundFiles/Combat/Cue_TutorialCombat_LateAttack.Cue_TutorialCombat_LateAttack" 1.0 1.0 0.0 0))
              (LocalVariables|SetAudioComponent _returnvalue_2)))
          (Utilities|Time|SetTimerbyFunctionName 0 "StartCombat" (+ (Variables|/Script/Engine.SoundBase|GetDuration (Variables|/Script/Engine.AudioComponent|GetSound (LocalVariables|GetAudioComponent))) 2.0)))))))