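; BP_PuzzlePawn is a puzzle pawn that the player controller temporarily possesses to give the player alternate controls.
; TriggerEvent stores the player reference, possesses the pawn and plays an enter sound, while IA_Interact calls ExitFocusEvent, repossesses the stored player and plays an exit sound.
; BeginPlay starts the pawn's environmental audio.
; PuzzleComplete only sets a completion flag, and no puzzle logic appears in these graphs.
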(event Input|EnhancedActionEvents|EnhancedInputActionIA_Interact
  (params (ActionValue :type Boolean) (ElapsedSeconds :type Float%20%28double-precision%29) (TriggeredSeconds :type Float%20%28double-precision%29) (InputAction :type Input%20Action%20Object%20Reference :default "/Game/ThirdPerson/Input/Actions/IA_Interact.IA_Interact"))
  (:Started
    (CallFunction|ExitFocusEvent 2.0)
    (CallFunction|RepossessPlayer)
    (Audio|PlaySound2D "/Game/SpookyGame/Audio/All_Rooms/SFX/SFX_Exit_AltCTRL_Cue.SFX_Exit_AltCTRL_Cue" 1.0 1.0 0.0 0 0)
    (Development|PrintString "Exiting alt controls" true true "(R=1.000000,G=0.332539,B=0.000000,A=1.000000)")))

(event EventBeginPlay
  (Audio|Components|Audio|SetSound (Variables|Default|GetEnvironmentalAudio) (Variables|Default|GetEnvironmentalSound))
  (Audio|Components|Audio|Play (Variables|Default|GetEnvironmentalAudio) 0.0))

(event EventTriggerEvent
  (params (PlayerREF :type BP%20SG%20Player%20Object%20Reference))
  (Variables|Default|SetPlayer%20REF PlayerREF)
  (Pawn|Possess (Game|GetPlayerController 0) self)
  (Audio|PlaySound2D "/Game/SpookyGame/Audio/All_Rooms/SFX/SFX_Enter_AltCTRL.SFX_Enter_AltCTRL" 1.0 1.0 0.0 0 0)
  (Development|PrintString "Enter alt controls" true true "(R=0.548844,G=1.000000,B=0.000000,A=1.000000)"))

(fn ConstructionScript)

(fn PuzzleComplete
  (Variables|Default|SetIsPuzzleCompleted true))

(fn RepossessPlayer
  (Pawn|Possess (Game|GetPlayerController 0) (Variables|Default|GetPlayer%20REF)))