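; Radio puzzle pawn with two tuning knobs: A/D turn the left and Left/Right arrows the right.
; Tick steps each value between 0 and 180 while its key is held, with turning loops and a ping at the limits.
; Each value's distance from its target band selects one of two static loops or journal noise, raising another audio layer on target.
; DoOnce gates that reset each other make sounds switch only on zone changes.
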(event EventBeginPlay
  (|CallParentFunction))

(event Collision|EventActorBeginOverlap
  (params (OtherActor :type Actor%20Object%20Reference)))

(event EventTriggerEvent
  (params (PlayerREF :type BP%20SG%20Player%20Object%20Reference))
  (|CallParentFunction PlayerREF)
  (Audio|Components|Audio|Stop (Variables|Default|GetEnvironmentalAudio))
  (Development|PrintString "STOP PLAY"))

(event EventTick
  (params (DeltaSeconds :type Float%20%28single-precision%29))
  (bind _left_audio (Variables|Default|GetLeft_Audio))
  (bind _right_audio (Variables|Default|GetRight_Audio))
  (bind _right_audio2 (Variables|Default|GetRight_Audio2))
  (bind _left_audio2 (Variables|Default|GetLeft_Audio2))
  (bind _left_audio3 (Variables|Default|GetLeft_Audio3))
  (bind _left_value (Variables|Default|GetLeft_Value))
  (bind _right_audio3 (Variables|Default|GetRight_Audio3))
  (bind _right_value (Variables|Default|GetRight_Value))
  (Utilities|FlowControl|Sequence
    (:then_0
      (if (Variables|Default|GetIs_D_Pressed?)
        (Utilities|FlowControl|Sequence
          (:then_0
            (Utilities|FlowControl|DoOnce false :!label _label
              (:Completed
                (if (== (Variables|Default|GetLeft_Value) 0.0)
                  (Audio|Components|Audio|SetSound (Variables|Default|GetLeft_Audio) "/Game/SpookyGame/Audio/Captain/SFX/SFX_Knob_Turn_Loop.SFX_Knob_Turn_Loop")
                  (goto _label_2 Reset)))))
          (:then_1
            (if (== (Variables|Default|GetLeft_Value) 1.8e+02)
              (Utilities|FlowControl|DoOnce false :!label _label_2
                (:Completed
                  (Audio|Components|Audio|SetSound _left_audio "/Engine/EngineSounds/1kSineTonePing.1kSineTonePing")
                  (Audio|Components|Audio|Play _left_audio 0.0)
                  (Utilities|FlowControl|Sequence
                    (:then_0
                      (goto _label Reset))
                    (:then_1
                      (goto _label_3 Reset)))))
              (else
                (bind _result (Math|Float|IncrementFloat (Variables|Default|GetLeft_Value))
                  (:%20%20
                    (Development|PrintString (Utilities|String|ToString(Float) _result))))))))
        (elif (Variables|Default|GetIs_A_Pressed?)
          (Utilities|FlowControl|Sequence
            (:then_0
              (Utilities|FlowControl|DoOnce false :!label _label_3
                (:Completed
                  (if (== (Variables|Default|GetLeft_Value) 1.8e+02)
                    (Audio|Components|Audio|SetSound (Variables|Default|GetLeft_Audio) "/Game/SpookyGame/Audio/Captain/SFX/SFX_Knob_Turn_Loop.SFX_Knob_Turn_Loop")
                    (goto _label_2 Reset)))))
            (:then_1
              (if (== (Variables|Default|GetLeft_Value) 0.0)
                (goto _label_2)
                (else
                  (bind _result_2 (Math|Float|DecrementFloat (Variables|Default|GetLeft_Value))
                    (:%20%20
                      (Development|PrintString (Utilities|String|ToString(Float) _result_2)))))))))))
    (:then_1
      (if (Variables|Default|GetIs_Right_Pressed?)
        (Utilities|FlowControl|Sequence
          (:then_0
            (Utilities|FlowControl|DoOnce false :!label _label_4
              (:Completed
                (if (== (Variables|Default|GetRight_Value) 0.0)
                  (Audio|Components|Audio|SetSound (Variables|Default|GetRight_Audio) "/Game/SpookyGame/Audio/Captain/SFX/SFX_Knob_Turn_Loop.SFX_Knob_Turn_Loop")
                  (goto _label_5 Reset)))))
          (:then_1
            (if (== (Variables|Default|GetRight_Value) 1.8e+02)
              (Utilities|FlowControl|DoOnce false :!label _label_5
                (:Completed
                  (Audio|Components|Audio|SetSound _right_audio "/Engine/EngineSounds/1kSineTonePing.1kSineTonePing")
                  (Audio|Components|Audio|Play _right_audio 0.0)
                  (Utilities|FlowControl|Sequence
                    (:then_0
                      (goto _label_4 Reset))
                    (:then_1
                      (goto _label_6 Reset)))))
              (else
                (bind _result_3 (Math|Float|IncrementFloat (Variables|Default|GetRight_Value))
                  (:%20%20
                    (Development|PrintString (Utilities|String|ToString(Float) _result_3))))))))
        (elif (Variables|Default|GetIs_Left_Pressed?)
          (Utilities|FlowControl|Sequence
            (:then_0
              (Utilities|FlowControl|DoOnce false :!label _label_6
                (:Completed
                  (if (== (Variables|Default|GetRight_Value) 1.8e+02)
                    (Audio|Components|Audio|SetSound (Variables|Default|GetRight_Audio) "/Game/SpookyGame/Audio/Captain/SFX/SFX_Knob_Turn_Loop.SFX_Knob_Turn_Loop")
                    (goto _label_5 Reset)))))
            (:then_1
              (if (== (Variables|Default|GetRight_Value) 0.0)
                (goto _label_5)
                (else
                  (bind _result_4 (Math|Float|DecrementFloat (Variables|Default|GetRight_Value))
                    (:%20%20
                      (Development|PrintString (Utilities|String|ToString(Float) _result_4)))))))))))
    (:then_2
      (if (not (== (Variables|Default|GetLeft_Value) 9e+01))
        (if (Math|Float|InRange(Float) (Variables|Default|GetLeft_Value) 38.0 48.0)
          (Utilities|FlowControl|Sequence
            (:then_0
              (Utilities|FlowControl|DoOnce false :!label _label_7
                (:Completed
                  (Utilities|FlowControl|Sequence
                    (:then_0
                      (Audio|Components|Audio|SetSound _left_audio2 "/Game/SpookyGame/Audio/Captain/UI/UI_Radio_Journal_Noise_Loop.UI_Radio_Journal_Noise_Loop")
                      (Audio|Components|Audio|Play _left_audio2 0.0 :!label _label_8))
                    (:then_1
                      (goto _label_11 Reset))
                    (:then_2
                      (goto _label_9 Reset))))))
            (:then_1
              (Audio|Components|Audio|SetVolumeMultiplier _left_audio3 0.5 :!class /Script/Engine.AudioComponent)))
          (elif (Math|Float|InRange(Float) (Variables|Default|GetLeft_Value) 23.0 63.0)
            (Utilities|FlowControl|DoOnce false :!label _label_9
              (:Completed
                (Utilities|FlowControl|Sequence
                  (:then_0
                    (Audio|Components|Audio|SetSound _left_audio2 "/Game/SpookyGame/Audio/Captain/SFX/SFX_Radio_Static_Loop_02.SFX_Radio_Static_Loop_02")
                    (goto _label_8))
                  (:then_1
                    (goto _label_11 Reset))
                  (:then_2
                    (goto _label_7 Reset))
                  (:then_3
                    (Audio|Components|Audio|SetVolumeMultiplier _left_audio3 0.0001 :!class /Script/Engine.AudioComponent :!label _label_10)))))
            (elif (or (< _left_value 23.0) (> _left_value 63.0))
              (Utilities|FlowControl|DoOnce false :!label _label_11
                (:Completed
                  (Utilities|FlowControl|Sequence
                    (:then_0
                      (Audio|Components|Audio|SetSound _left_audio2 "/Game/SpookyGame/Audio/Captain/SFX/SFX_Radio_Static_Loop_01.SFX_Radio_Static_Loop_01")
                      (goto _label_8))
                    (:then_1
                      (goto _label_7 Reset))
                    (:then_2
                      (goto _label_9 Reset))
                    (:then_3
                      (goto _label_10))))))))))
    (:then_3
      (if (not (== (Variables|Default|GetRight_Value) 9e+01))
        (if (Math|Float|InRange(Float) (Variables|Default|GetRight_Value) 116.0 126.0)
          (Utilities|FlowControl|Sequence
            (:then_0
              (Utilities|FlowControl|DoOnce false :!label _label_12
                (:Completed
                  (Utilities|FlowControl|Sequence
                    (:then_0
                      (Audio|Components|Audio|SetSound _right_audio2 "/Game/SpookyGame/Audio/Captain/UI/UI_Radio_Journal_Noise_Loop.UI_Radio_Journal_Noise_Loop")
                      (Audio|Components|Audio|SetVolumeMultiplier _right_audio2 1.0 :!class /Script/Engine.AudioComponent)
                      (Audio|Components|Audio|Play _right_audio2 0.0 :!label _label_13))
                    (:then_1
                      (goto _label_17 Reset))
                    (:then_2
                      (goto _label_14 Reset))))))
            (:then_1
              (Audio|Components|Audio|SetVolumeMultiplier _right_audio3 0.5 :!class /Script/Engine.AudioComponent)))
          (elif (Math|Float|InRange(Float) (Variables|Default|GetRight_Value) 101.0 141.0)
            (Utilities|FlowControl|DoOnce false :!label _label_14
              (:Completed
                (Utilities|FlowControl|Sequence
                  (:then_0
                    (Audio|Components|Audio|SetSound _right_audio2 "/Game/SpookyGame/Audio/Captain/SFX/SFX_Radio_Static_Loop_02.SFX_Radio_Static_Loop_02")
                    (Audio|Components|Audio|SetVolumeMultiplier _right_audio2 0.5 :!class /Script/Engine.AudioComponent :!label _label_15)
                    (goto _label_13))
                  (:then_1
                    (goto _label_17 Reset))
                  (:then_2
                    (goto _label_12 Reset))
                  (:then_3
                    (Audio|Components|Audio|SetVolumeMultiplier _right_audio3 0.0001 :!class /Script/Engine.AudioComponent :!label _label_16)))))
            (elif (or (< _right_value 101.0) (> _right_value 141.0))
              (Utilities|FlowControl|DoOnce false :!label _label_17
                (:Completed
                  (Utilities|FlowControl|Sequence
                    (:then_0
                      (Audio|Components|Audio|SetSound _right_audio2 "/Game/SpookyGame/Audio/Captain/SFX/SFX_Radio_Static_Loop_01.SFX_Radio_Static_Loop_01")
                      (goto _label_15))
                    (:then_1
                      (goto _label_12 Reset))
                    (:then_2
                      (goto _label_14 Reset))
                    (:then_3
                      (goto _label_16))))))))))))

(event Input|KeyboardEvents|Right
  (params (Key :type Key%20Structure :default "None"))
  (bind _right_audio (Variables|Default|GetRight_Audio))
  (:Pressed
    (if (not (== (Variables|Default|GetRight_Value) 1.8e+02))
      (Variables|Default|SetIs_Right_Pressed? true)
      (Audio|Components|Audio|Play _right_audio 0.0)))
  (:Released
    (Variables|Default|SetIs_Right_Pressed? false)
    (Audio|Components|Audio|Stop _right_audio)))

(event Input|KeyboardEvents|A
  (params (Key :type Key%20Structure :default "None"))
  (bind _left_audio (Variables|Default|GetLeft_Audio))
  (:Pressed
    (if (not (== (Variables|Default|GetLeft_Value) 0.0))
      (Variables|Default|SetIs_A_Pressed? true)
      (Audio|Components|Audio|Play _left_audio 0.0)))
  (:Released
    (Variables|Default|SetIs_A_Pressed? false)
    (Audio|Components|Audio|Stop _left_audio)))

(event Input|KeyboardEvents|D
  (params (Key :type Key%20Structure :default "None"))
  (bind _left_audio (Variables|Default|GetLeft_Audio))
  (:Pressed
    (if (not (== (Variables|Default|GetLeft_Value) 1.8e+02))
      (Variables|Default|SetIs_D_Pressed? true)
      (Audio|Components|Audio|Play _left_audio 0.0)))
  (:Released
    (Variables|Default|SetIs_D_Pressed? false)
    (Audio|Components|Audio|Stop _left_audio)))

(event Input|KeyboardEvents|Left
  (params (Key :type Key%20Structure :default "None"))
  (bind _right_audio (Variables|Default|GetRight_Audio))
  (:Pressed
    (if (not (== (Variables|Default|GetRight_Value) 0.0))
      (Variables|Default|SetIs_Left_Pressed? true)
      (Audio|Components|Audio|Play _right_audio 0.0)))
  (:Released
    (Variables|Default|SetIs_Left_Pressed? false)
    (Audio|Components|Audio|Stop _right_audio)))

(fn ConstructionScript
  (|CallParentFunction))